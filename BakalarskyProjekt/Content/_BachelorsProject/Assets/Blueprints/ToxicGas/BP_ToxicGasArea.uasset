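; BP_ToxicGasArea is a hazard volume that repeatedly damages an actor with a HeathComponent inside its box.
; After a short delay on overlap, it plays a one-time bubbling sound at world origin, adds a particle effect and starts a looping damage timer on that actor, stored as the single target.
; End overlap clears the timer but cannot cancel a pending delay.
; An unconnected radial-damage debug chain remains in the graph.
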(event OnComponentBeginOverlap(Box)
  (params (OverlappedComponent :type Primitive%20Component%20Object%20Reference) (OtherActor :type Actor%20Object%20Reference) (OtherComp :type Primitive%20Component%20Object%20Reference) (OtherBodyIndex :type Integer) (bFromSweep :type Boolean) (SweepResult :type Hit%20Result%20Structure%20%28by%20ref%29))
  (Utilities|IsValid (Actor|GetComponentbyClass OtherActor "/Game/_BachelorsProject/Components/HeathComponent.HeathComponent_C")
    (:Is%20Valid
      (Utilities|FlowControl|Delay 2.0)
      (Utilities|FlowControl|Sequence
        (:then_0
          ;[0 0.8229 0.5852 0.5] Sound effect
          (if (not (Variables|Default|GetSound%20is%20playing?))
            (Audio|PlaySoundatLocation "/Game/_BachelorsProject/Assets/soundEffects/heavy-bubbles-35889_Cue.heavy-bubbles-35889_Cue" "0, 0, 0" "0, 0, 0" 4.0 3.0 0.0 0 0 0 0)
            (Variables|Default|SetSound%20is%20playing? true)))
        (:then_1
          (AddComponent|AddParticleSystemComponent false)
          (Variables|Default|SetTarget_Char OtherActor)
          (Utilities|Time|SetTimerbyFunctionName 0 "ApplyDamage" 1.0 true)
          (CallFunction|ApplyDamage))))))

(event OnComponentEndOverlap(Box)
  (params (OverlappedComponent :type Primitive%20Component%20Object%20Reference) (OtherActor :type Actor%20Object%20Reference) (OtherComp :type Primitive%20Component%20Object%20Reference) (OtherBodyIndex :type Integer))
  (Utilities|IsValid (Actor|GetComponentbyClass OtherActor "/Game/_BachelorsProject/Components/HeathComponent.HeathComponent_C")
    (:Is%20Valid
      (Utilities|Time|ClearTimerbyFunctionName 0 "ApplyDamage"))))

(fn ConstructionScript)

(fn ApplyDamage
  (bind _returnvalue (Game|Damage|ApplyDamage (Variables|Default|GetTarget_Char) 1e+01 0 0))
  (Development|PrintString (Utilities|String|ToString(Float) _returnvalue) true true "(R=0.028845,G=0.116165,B=1.000000,A=1.000000)" 1e+01))