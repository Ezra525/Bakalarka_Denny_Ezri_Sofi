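; Puzzle box that the crab character can push, sliding its cube sideways along a Timeline when the pickup input is pressed.
; Overlapping the Box trigger with BP_crabcollision enables player input on the actor, and leaving disables it.
; Until pushed, a box tagged "first box" shows internal dialogue through the game mode on Widgetrange overlap, with text depending on whether the player is the original character.
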(event OnComponentBeginOverlap(Box)
  (params (OverlappedComponent :type Primitive%20Component%20Object%20Reference) (OtherActor :type Actor%20Object%20Reference) (OtherComp :type Primitive%20Component%20Object%20Reference) (OtherBodyIndex :type Integer) (bFromSweep :type Boolean) (SweepResult :type Hit%20Result%20Structure%20%28by%20ref%29))
  (bind _asbp_crabcollision (Utilities|Casting|CastToBP_crabcollision OtherActor)
    (:then
      (if (== _asbp_crabcollision OtherActor)
        (Input|EnableInput (Game|GetPlayerController 0))))
    (:CastFailed
      (Development|PrintString "Not A crab on box" true true "(R=1.000000,G=0.905883,B=0.000000,A=1.000000)"))))

(event OnComponentEndOverlap(Box)
  (params (OverlappedComponent :type Primitive%20Component%20Object%20Reference) (OtherActor :type Actor%20Object%20Reference) (OtherComp :type Primitive%20Component%20Object%20Reference) (OtherBodyIndex :type Integer))
  (bind _asbp_crabcollision (Utilities|Casting|CastToBP_crabcollision OtherActor))
  (if (== _asbp_crabcollision OtherActor)
    (Input|DisableInput (Game|GetPlayerController 0))))

(event OnComponentBeginOverlap(widgetrange)
  (params (OverlappedComponent :type Primitive%20Component%20Object%20Reference) (OtherActor :type Actor%20Object%20Reference) (OtherComp :type Primitive%20Component%20Object%20Reference) (OtherBodyIndex :type Integer) (bFromSweep :type Boolean) (SweepResult :type Hit%20Result%20Structure%20%28by%20ref%29))
  (if (== (Game|GetPlayerCharacter 0) (Variables|/Game/ThirdPerson/Blueprints/BP_ThirdPersonGameMode.BP_ThirdPersonGameMode_C|GetOriginalTypek (Variables|Default|GetAs%20BP%20Third%20Person%20Game%20Mode)))
    (if (not (Variables|Default|Getdone%20box))
      (if (Actor|ActorHasTag self "first box")
        (Default|CallInternalDialogue (Variables|Default|GetAs%20BP%20Third%20Person%20Game%20Mode) (Variables|Default|GetInternal%20Dialogue%20Parazit))))
    (elif (not (Variables|Default|Getdone%20box))
      (if (Actor|ActorHasTag self "first box")
        (Default|CallInternalDialogue (Variables|Default|GetAs%20BP%20Third%20Person%20Game%20Mode) (Variables|Default|GetInternal%20Dialogue%20Crab))))))

(event OnComponentEndOverlap(widgetrange)
  (params (OverlappedComponent :type Primitive%20Component%20Object%20Reference) (OtherActor :type Actor%20Object%20Reference) (OtherComp :type Primitive%20Component%20Object%20Reference) (OtherBodyIndex :type Integer))
  (if (== OtherActor (Game|GetPlayerCharacter 0))
    (Default|CallInternalDialogue (Variables|Default|GetAs%20BP%20Third%20Person%20Game%20Mode) (Variables|Default|GetEmpty%20text))))

(event Custom|push%20box
  (Utilities|FlowControl|FlipFlop
    (:A
      (bind _doorrotattion (Timeline|Timeline Play)
        (:Update
          (Transformation|SetRelativeLocation (Variables|Default|GetCube) (Math|Vector|MakeVector 0.0 (Math|Float|Lerp 0.0 2e+02 _doorrotattion) 0.0) false false)
          (Variables|Default|Setdone%20box true))))))

(event Input|EnhancedActionEvents|EnhancedInputActionIA_pickup
  (params (ActionValue :type Boolean) (ElapsedSeconds :type Float%20%28double-precision%29) (TriggeredSeconds :type Float%20%28double-precision%29) (InputAction :type Input%20Action%20Object%20Reference :default "/Game/ThirdPerson/Input/Actions/IA_pickup.IA_pickup"))
  (CallFunction|PushBox))

(event EventBeginPlay
  (bind _asbp_third_person_game_mode (Utilities|Casting|CastToBP_ThirdPersonGameMode (Game|GetGameMode)))
  (Variables|Default|SetAs%20BP%20Third%20Person%20Game%20Mode _asbp_third_person_game_mode))

(fn ConstructionScript)