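; Electricity generator for the power-on puzzle that takes a charge from an eel.
; When an actor tagged "eel" overlaps component R while its MamElektriku (has electricity) flag is set, the generator applies damage to itself, though this graph has no damage handler.
; It then clears the eel's flag, swaps the eel's mesh material and reveals its Sphere, which is hidden at BeginPlay.
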(event OnComponentBeginOverlap(r)
  (params (OverlappedComponent :type Primitive%20Component%20Object%20Reference) (OtherActor :type Actor%20Object%20Reference) (OtherComp :type Primitive%20Component%20Object%20Reference) (OtherBodyIndex :type Integer) (bFromSweep :type Boolean) (SweepResult :type Hit%20Result%20Structure%20%28by%20ref%29))
  ;[0.15 0.15 0.15 0.5] Charge generator
  (if (Actor|ActorHasTag OtherActor "eel")
    (bind _asbp_eel (Utilities|Casting|CastToBP_eel OtherActor))
    (if (Variables|/Game/_BachelorsProject/Assets/Blueprints/AI/fish/BP_eel.BP_eel_C|GetMam%20elektriku _asbp_eel)
      (Game|Damage|ApplyDamage self 1e+01 0 0)
      (Variables|/Game/_BachelorsProject/Assets/Blueprints/AI/fish/BP_eel.BP_eel_C|SetMam%20elektriku _asbp_eel false)
      (Rendering|Material|SetMaterial (Variables|/Script/Engine.Character|GetMesh _asbp_eel) 0 "/Game/Fab/eel/pyjama_shark_mat.pyjama_shark_mat")
      (Development|SetHiddeninGame (Variables|Default|GetSphere) false false))))

(event EventBeginPlay
  ;[0.15 0.15 0.15 0.5] Hide sphere
  (Development|SetHiddeninGame (Variables|Default|GetSphere) true false))

(fn ConstructionScript)