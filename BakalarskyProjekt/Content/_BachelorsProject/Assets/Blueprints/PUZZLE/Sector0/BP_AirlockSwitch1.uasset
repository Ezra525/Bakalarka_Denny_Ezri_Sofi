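; Airlock switch for the Sector 0 puzzle that lets the player open a wall.
; Box overlaps toggle the actor's input, so the pickup action can call CallSector0 on the third-person game mode and mark the switch done.
; Until done, player entry triggers one of two internal dialogues depending on whether the current character is OriginalTypek.
; Player exit always sends the Thoughts value to the dialogue call.
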(event OnComponentBeginOverlap(Box)
  (params (OverlappedComponent :type Primitive%20Component%20Object%20Reference) (OtherActor :type Actor%20Object%20Reference) (OtherComp :type Primitive%20Component%20Object%20Reference) (OtherBodyIndex :type Integer) (bFromSweep :type Boolean) (SweepResult :type Hit%20Result%20Structure%20%28by%20ref%29))
  (bind _returnvalue (Game|GetPlayerCharacter 0))
  ;[0.3115 1 0 0.5] Internal Dialogue
  (Input|EnableInput (Game|GetPlayerController 0))
  (if (== _returnvalue OtherActor)
    (if (== _returnvalue (Variables|/Game/ThirdPerson/Blueprints/BP_ThirdPersonGameMode.BP_ThirdPersonGameMode_C|GetOriginalTypek (Variables|Default|GetAs%20BP%20Third%20Person%20Game%20Mode)))
      (if (not (Variables|Default|Getdone))
        (Default|CallInternalDialogue (Variables|Default|GetAs%20BP%20Third%20Person%20Game%20Mode) (Variables|Default|Get1)))
      (elif (not (Variables|Default|Getdone))
        (Default|CallInternalDialogue (Variables|Default|GetAs%20BP%20Third%20Person%20Game%20Mode) (Variables|Default|Get2))))))

(event OnComponentEndOverlap(Box)
  (params (OverlappedComponent :type Primitive%20Component%20Object%20Reference) (OtherActor :type Actor%20Object%20Reference) (OtherComp :type Primitive%20Component%20Object%20Reference) (OtherBodyIndex :type Integer))
  ;[0.3115 1 0 0.5] Internal Dialogue
  (Input|DisableInput (Game|GetPlayerController 0))
  (if (== OtherActor (Game|GetPlayerCharacter 0))
    (Default|CallInternalDialogue (Variables|Default|GetAs%20BP%20Third%20Person%20Game%20Mode) (Variables|Default|GetThoughts))))

(event Input|EnhancedActionEvents|EnhancedInputActionIA_pickup
  (params (ActionValue :type Boolean) (ElapsedSeconds :type Float%20%28double-precision%29) (TriggeredSeconds :type Float%20%28double-precision%29) (InputAction :type Input%20Action%20Object%20Reference :default "/Game/ThirdPerson/Input/Actions/IA_pickup.IA_pickup"))
  ;[1 0.28 0 0.5] Open wall
  (Default|CallSector0 (Variables|Default|GetAs%20BP%20Third%20Person%20Game%20Mode))
  (Variables|Default|Setdone true))

(event EventBeginPlay
  ;[0.474 0 1 0.5] Set variables
  (bind _asbp_third_person_game_mode (Utilities|Casting|CastToBP_ThirdPersonGameMode (Game|GetGameMode)))
  (Variables|Default|SetAs%20BP%20Third%20Person%20Game%20Mode _asbp_third_person_game_mode))

(fn ConstructionScript)