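; BP_glass_wall is a puzzle glass wall that slides downward when triggered through the game mode.
; On BeginPlay it binds its move event to BP_ThirdPersonGameMode.
; The event plays a timeline that adds a lerped downward offset to the cube every update, so movement accumulates rather than interpolating to a fixed endpoint.
; A flag lets the wall's sound play only once at its location.
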(event Custom|move
  (Utilities|FlowControl|Sequence
    (:then_0
      (bind _elevator_up (Timeline|Timeline Play)
        (:Update
          (Transformation|AddRelativeLocation (Variables|Default|GetCube) (Math|Vector|Lerp(Vector) "0, 0, 0" "0.000000,0.000000,-200.000000" _elevator_up) false false))))
    (:then_1
      (if (not (Variables|Default|GetSound%20is%20playing?))
        (Audio|PlaySoundatLocation "/Game/_BachelorsProject/Assets/soundEffects/glass_wall_Cue.glass_wall_Cue" (Transformation|GetWorldLocation (Variables|Default|GetDefaultSceneRoot)) "0, 0, 0" 1.0 1.0 0.0 0 0 0 0)
        (Variables|Default|SetSound%20is%20playing? true)))))

(event EventBeginPlay
  (bind _asbp_third_person_game_mode (Utilities|Casting|CastToBP_ThirdPersonGameMode (Game|GetGameMode)))
  (EventDispatchers|BindEventtoGlassWall _asbp_third_person_game_mode (delegate Custom|move)))

(fn ConstructionScript)