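; Puzzle elevator actor that drops 20 units and triggers the player's internal dialogue.
; On BeginPlay it registers with the third-person game mode's elevator-called event and constructs a "what was that" widget.
; Its move event shifts it down instantly, then sends two delayed lines through the game mode unless a done flag is set.
; The widget display and the setting of that flag are disconnected, so neither runs.
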(event Custom|move
  (Transformation|SetActorLocation (- (Transformation|GetWorldLocation (Variables|Default|GetDefaultSceneRoot self)) "0.000000,0.000000,20.000000") false false)
  (if (not (Variables|Default|Getalreadzhotovo))
    (Utilities|FlowControl|Delay 1.0)
    (Default|CallInternalDialogue (Variables|Default|GetAs%20BP%20Third%20Person%20Game%20Mode) (Variables|Default|GetInternal%20Dialogue))
    (Utilities|FlowControl|Delay 2.0)
    (Default|CallInternalDialogue (Variables|Default|GetAs%20BP%20Third%20Person%20Game%20Mode) (Variables|Default|GetThoughts))))

(event EventBeginPlay
  (Utilities|FlowControl|Sequence
    (:then_0
      (bind _asbp_third_person_game_mode (Utilities|Casting|CastToBP_ThirdPersonGameMode (Game|GetGameMode)))
      (Variables|Default|SetAs%20BP%20Third%20Person%20Game%20Mode _asbp_third_person_game_mode)
      (EventDispatchers|BindEventtoElevatorCalled (Variables|Default|GetAs%20BP%20Third%20Person%20Game%20Mode) (EventDispatchers|CreateEvent :!event Custom|move)))
    (:then_1
      (bind _returnvalue (Game|ConstructObjectfromClass "/Game/_BachelorsProject/Assets/widgets/first_room/P_whatwasthat.P_whatwasthat_C"))
      (Variables|Default|Setwhat%20was%20that%20 _returnvalue))))

(fn ConstructionScript)