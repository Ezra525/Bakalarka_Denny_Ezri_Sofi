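; Airlock door for the Sector 3 puzzle that drops downward when the game mode signals it to open.
; On BeginPlay it binds its move event to the third-person game mode's airlock door event.
; Each call lowers the actor 100 units in one unswept step, with no interpolation.
; A flag limits the opening sound to the first call, while the movement repeats on every call.
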(event Custom|move
  (Utilities|FlowControl|Sequence
    (:then_0
      (Transformation|SetActorLocation (- (Transformation|GetWorldLocation (Variables|Default|GetDefaultSceneRoot)) "0.000000,0.000000,100.000000") false false))
    (:then_1
      (if (not (Variables|Default|GetSound%20is%20playing?))
        (Audio|PlaySoundatLocation "/Game/_BachelorsProject/Assets/soundEffects/Airlock_opening_Cue.Airlock_opening_Cue" (Transformation|GetWorldLocation (Variables|Default|GetDefaultSceneRoot)) "0, 0, 0" 1.0 1.0 0.0 0 0 0 0)
        (Variables|Default|SetSound%20is%20playing? true)))))

(event EventBeginPlay
  (bind _asbp_third_person_game_mode (Utilities|Casting|CastToBP_ThirdPersonGameMode (Game|GetGameMode)))
  (EventDispatchers|BindEventtoAirLockDoor _asbp_third_person_game_mode (delegate Custom|move)))

(fn ConstructionScript)