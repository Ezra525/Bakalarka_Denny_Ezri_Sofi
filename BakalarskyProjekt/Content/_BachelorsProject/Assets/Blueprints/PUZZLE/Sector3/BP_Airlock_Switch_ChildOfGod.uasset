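; Airlock switch for the Sector 3 puzzle, which lets the player trigger an airlock door while standing near it.
; Overlapping the Box enables input from player controller 0, and leaving it disables input, without filtering the overlapping actor.
; The IA_pickup input action calls AirlockSwitch to signal the door; the opening logic is not in this Blueprint.
; Debug strings print on each event, and construction defers to the parent class.
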(event OnComponentBeginOverlap(Box)
  (params (OverlappedComponent :type Primitive%20Component%20Object%20Reference) (OtherActor :type Actor%20Object%20Reference) (OtherComp :type Primitive%20Component%20Object%20Reference) (OtherBodyIndex :type Integer) (bFromSweep :type Boolean) (SweepResult :type Hit%20Result%20Structure%20%28by%20ref%29))
  ;[0.3115 1 0 0.5] Internal Dialogue
  (Input|EnableInput (Game|GetPlayerController 0))
  (Development|PrintString "Input on"))

(event OnComponentEndOverlap(Box)
  (params (OverlappedComponent :type Primitive%20Component%20Object%20Reference) (OtherActor :type Actor%20Object%20Reference) (OtherComp :type Primitive%20Component%20Object%20Reference) (OtherBodyIndex :type Integer))
  ;[0.3115 1 0 0.5] Internal Dialogue
  (Input|DisableInput (Game|GetPlayerController 0))
  (Development|PrintString "input off"))

(event Input|EnhancedActionEvents|EnhancedInputActionIA_pickup
  (params (ActionValue :type Boolean) (ElapsedSeconds :type Float%20%28double-precision%29) (TriggeredSeconds :type Float%20%28double-precision%29) (InputAction :type Input%20Action%20Object%20Reference :default "/Game/ThirdPerson/Input/Actions/IA_pickup.IA_pickup"))
  ;[1 0.28 0 0.5] Open wall
  (Default|CallAirlockSwitch)
  (Development|PrintString "calling airlock door"))

(fn ConstructionScript
  (|CallParentFunction))