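; Pickup actor for an iron item ("zelezo") in the ventilation puzzle, removed when the player picks it up.
; Crab's begin-overlap event checks whether the other actor is this one, then enables input and sets the proximity flag SomPriKluci, printing debug messages.
; Any end overlap on Crab disables input and clears the flag.
; The IA_pickup input action destroys the actor while the flag is set.
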(event OnActorBeginOverlap(crab)
  (params (OverlappedActor :type Actor%20Object%20Reference) (OtherActor :type Actor%20Object%20Reference))
  (if (== OtherActor self)
    (Development|PrintString "mam imput")
    (Input|EnableInput (Game|GetPlayerController 0))
    (Variables|Default|Setsom%20pri%20kluci true)
    (else
      (Development|PrintString "nemam imput"))))

(event OnActorEndOverlap(crab)
  (params (OverlappedActor :type Actor%20Object%20Reference) (OtherActor :type Actor%20Object%20Reference))
  (Input|DisableInput (Game|GetPlayerController 0))
  (Variables|Default|Setsom%20pri%20kluci false))

(event Input|EnhancedActionEvents|EnhancedInputActionIA_pickup
  (params (ActionValue :type Boolean) (ElapsedSeconds :type Float%20%28double-precision%29) (TriggeredSeconds :type Float%20%28double-precision%29) (InputAction :type Input%20Action%20Object%20Reference :default "/Game/ThirdPerson/Input/Actions/IA_pickup.IA_pickup"))
  (:Triggered
    (if (Variables|Default|Getsom%20pri%20kluci)
      (Actor|DestroyActor))))

(event EventBeginPlay)

(event Collision|EventActorBeginOverlap
  (params (OtherActor :type Actor%20Object%20Reference)))

(event EventTick
  (params (DeltaSeconds :type Float%20%28single-precision%29)))

(fn ConstructionScript)