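; BP_ventilacia is a ventilation fan puzzle obstacle that spins with looping-style Timeline rotation and attached fan noise.
; Destruction of the referenced Key actor flags that the player has the iron ("zelezo").
; An overlap trigger enables input for actors tagged "Crab", so pickup with the iron stops the fan and sound, disables fan collision and reveals two hidden components.
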(event OnDestroyed(Key)
  (params (DestroyedActor :type Actor%20Object%20Reference))
  (Variables|Default|Setmamzelezo true)
  (Development|PrintString "mam zelezo"))

(event OnComponentBeginOverlap(r)
  (params (OverlappedComponent :type Primitive%20Component%20Object%20Reference) (OtherActor :type Actor%20Object%20Reference) (OtherComp :type Primitive%20Component%20Object%20Reference) (OtherBodyIndex :type Integer) (bFromSweep :type Boolean) (SweepResult :type Hit%20Result%20Structure%20%28by%20ref%29))
  (if (Actor|ActorHasTag OtherActor "Crab")
    (Variables|Default|Setsom%20pri%20ventilacii true)
    (Input|EnableInput (Game|GetPlayerController 0))))

(event OnComponentEndOverlap(r)
  (params (OverlappedComponent :type Primitive%20Component%20Object%20Reference) (OtherActor :type Actor%20Object%20Reference) (OtherComp :type Primitive%20Component%20Object%20Reference) (OtherBodyIndex :type Integer))
  (Variables|Default|Setsom%20pri%20ventilacii false)
  (Input|DisableInput (Game|GetPlayerController 0)))

(event Input|EnhancedActionEvents|EnhancedInputActionIA_pickup
  (params (ActionValue :type Boolean) (ElapsedSeconds :type Float%20%28double-precision%29) (TriggeredSeconds :type Float%20%28double-precision%29) (InputAction :type Input%20Action%20Object%20Reference :default "/Game/ThirdPerson/Input/Actions/IA_pickup.IA_pickup"))
  (if (Variables|Default|Getsom%20pri%20ventilacii)
    (if (Variables|Default|Getmamzelezo)
      (Utilities|FlowControl|Sequence
        (:then_0
          (bind _doorrotattion (Timeline|Timeline Stop)
            (:Update
              (Transformation|SetRelativeRotation (Variables|Default|Getventilacia) (Math|Rotator|MakeRotator (Math|Float|Lerp 0.0 3.6e+02 _doorrotattion) 0.0 0.0) false false))))
        (:then_1
          (Collision|SetCollisionEnabled (Variables|Default|Getventilacia) "NoCollision")
          (Rendering|SetVisibility (Variables|Default|Getrrrere) true false)
          (Audio|Components|Audio|Stop (stale EventBeginPlay _returnvalue)))))))

(event EventBeginPlay
  (bind _returnvalue (Audio|SpawnSoundAttached "/Game/_BachelorsProject/Assets/soundEffects/noisy-ventilation-fan-61273.noisy-ventilation-fan-61273" (Variables|Default|Getventilacia) "None" (Transformation|GetActorLocation) "0, 0, 0" "SnapToTargetIncludingScale" true 1.0 1.0 0.0 "/Game/_BachelorsProject/Assets/soundEffects/Atenuation/ventilation.ventilation" 0))
  (Rendering|SetVisibility (Variables|Default|Getrrrr) false false)
  (Collision|SetCollisionEnabled (Variables|Default|Getrrrr) "NoCollision")
  (Collision|SetCollisionEnabled (Variables|Default|Getventilacia) "QueryAndPhysics")
  (Variables|Default|Setmamzelezo false)
  (bind _doorrotattion (Timeline|Timeline Play)
    (:Update
      (Transformation|SetRelativeRotation (Variables|Default|Getventilacia) (Math|Rotator|MakeRotator (Math|Float|Lerp 0.0 3.6e+02 _doorrotattion) 0.0 0.0) false false))))

(fn ConstructionScript)