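; Elevator call trigger for a puzzle area: pressing the pickup input inside its box notifies the game mode that the elevator was called.
; Box overlap with the player character enables the actor's input, and leaving disables it.
; A separate widget range sends timed internal dialogue and interaction prompts through game mode calls until the elevator has been called.
; Control panel and press-E widgets are constructed at BeginPlay but never displayed here.
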(event OnComponentBeginOverlap(widgetrange)
  (params (OverlappedComponent :type Primitive%20Component%20Object%20Reference) (OtherActor :type Actor%20Object%20Reference) (OtherComp :type Primitive%20Component%20Object%20Reference) (OtherBodyIndex :type Integer) (bFromSweep :type Boolean) (SweepResult :type Hit%20Result%20Structure%20%28by%20ref%29))
  (if (== OtherActor (Game|GetPlayerCharacter 0))
    (if (not (Variables|Default|Getalreadydown))
      (Default|CallInternalDialogue (Variables|Default|GetAs%20BP%20Third%20Person%20Game%20Mode) (Variables|Default|GetInternal%20Dialogue))
      (Utilities|FlowControl|Delay 2.0)
      (Default|CallInternalDialogue (Variables|Default|GetAs%20BP%20Third%20Person%20Game%20Mode))
      (Variables|Default|Setedissapierd false)
      (Default|CallInteraction (Variables|Default|GetAs%20BP%20Third%20Person%20Game%20Mode) (Variables|Default|Getepress))
      (Utilities|FlowControl|Delay 2.0)
      (Default|CallInteraction (Variables|Default|GetAs%20BP%20Third%20Person%20Game%20Mode) (Variables|Default|GetInteraction))
      (Variables|Default|Setedissapierd true))))

(event OnComponentEndOverlap(widgetrange)
  (params (OverlappedComponent :type Primitive%20Component%20Object%20Reference) (OtherActor :type Actor%20Object%20Reference) (OtherComp :type Primitive%20Component%20Object%20Reference) (OtherBodyIndex :type Integer))
  (if (== OtherActor (Game|GetPlayerCharacter 0))
    (if (Variables|Default|Getedissapierd)
      (Default|CallInteraction (Variables|Default|GetAs%20BP%20Third%20Person%20Game%20Mode) (Variables|Default|GetInteraction)))))

(event OnComponentBeginOverlap(BoxCollision)
  (params (OverlappedComponent :type Primitive%20Component%20Object%20Reference) (OtherActor :type Actor%20Object%20Reference) (OtherComp :type Primitive%20Component%20Object%20Reference) (OtherBodyIndex :type Integer) (bFromSweep :type Boolean) (SweepResult :type Hit%20Result%20Structure%20%28by%20ref%29))
  (Utilities|Casting|CastToBP_ThirdPersonCharacter_Child OtherActor)
  (Input|EnableInput (Game|GetPlayerController 0)))

(event OnComponentEndOverlap(BoxCollision)
  (params (OverlappedComponent :type Primitive%20Component%20Object%20Reference) (OtherActor :type Actor%20Object%20Reference) (OtherComp :type Primitive%20Component%20Object%20Reference) (OtherBodyIndex :type Integer))
  (Input|DisableInput (Game|GetPlayerController 0)))

(event Input|EnhancedActionEvents|EnhancedInputActionIA_pickup
  (params (ActionValue :type Boolean) (ElapsedSeconds :type Float%20%28double-precision%29) (TriggeredSeconds :type Float%20%28double-precision%29) (InputAction :type Input%20Action%20Object%20Reference :default "/Game/ThirdPerson/Input/Actions/IA_pickup.IA_pickup"))
  (Default|CallElevatorCalled (Variables|Default|GetAs%20BP%20Third%20Person%20Game%20Mode))
  (Variables|Default|Setalreadydown true))

(event EventBeginPlay
  (Utilities|FlowControl|Sequence
    (:then_0
      (bind _asbp_third_person_game_mode (Utilities|Casting|CastToBP_ThirdPersonGameMode (Game|GetGameMode)))
      (Variables|Default|SetAs%20BP%20Third%20Person%20Game%20Mode _asbp_third_person_game_mode))
    (:then_1
      (bind _returnvalue (Game|ConstructObjectfromClass "/Game/_BachelorsProject/Assets/widgets/first_room/P_controlPanel.P_controlPanel_C"))
      (Variables|Default|SetcontrolPanelWidget _returnvalue))
    (:then_2
      (bind _returnvalue_2 (Game|ConstructObjectfromClass "/Game/_BachelorsProject/Assets/widgets/first_room/P_pressEto.P_pressEto_C"))
      (Variables|Default|Setpressewidget _returnvalue_2))))

(fn ConstructionScript)