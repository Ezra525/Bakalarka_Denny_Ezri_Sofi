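; BP_Lever is a puzzle lever that calls the game mode's glass wall function when the pickup input fires.
; Its box enables input on any actor overlap and disables it on exit.
; Player overlaps trigger internal dialogue through the game mode, varying by whether the character is OriginalTypek, with another call on exit.
; The Done flag silences entry dialogue after use but does not block repeat pulls.
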(event OnComponentBeginOverlap(Box)
  (params (OverlappedComponent :type Primitive%20Component%20Object%20Reference) (OtherActor :type Actor%20Object%20Reference) (OtherComp :type Primitive%20Component%20Object%20Reference) (OtherBodyIndex :type Integer) (bFromSweep :type Boolean) (SweepResult :type Hit%20Result%20Structure%20%28by%20ref%29))
  (bind _returnvalue (Game|GetPlayerCharacter 0))
  (Input|EnableInput (Game|GetPlayerController 0))
  (if (== _returnvalue OtherActor)
    (if (== _returnvalue (Variables|/Game/ThirdPerson/Blueprints/BP_ThirdPersonGameMode.BP_ThirdPersonGameMode_C|GetOriginalTypek (stale EventBeginPlay _asbp_third_person_game_mode)))
      (if (not (Variables|Default|Getdone))
        (Default|CallInternalDialogue (stale EventBeginPlay _asbp_third_person_game_mode) (Variables|Default|Get1)))
      (elif (not (Variables|Default|Getdone))
        (Default|CallInternalDialogue (stale EventBeginPlay _asbp_third_person_game_mode) (Variables|Default|Get2))))))

(event OnComponentEndOverlap(Box)
  (params (OverlappedComponent :type Primitive%20Component%20Object%20Reference) (OtherActor :type Actor%20Object%20Reference) (OtherComp :type Primitive%20Component%20Object%20Reference) (OtherBodyIndex :type Integer))
  (Input|DisableInput (Game|GetPlayerController 0))
  (if (== OtherActor (Game|GetPlayerCharacter 0))
    (Default|CallInternalDialogue (stale EventBeginPlay _asbp_third_person_game_mode) (Variables|Default|GetThoughts))))

(event Input|EnhancedActionEvents|EnhancedInputActionIA_pickup
  (params (ActionValue :type Boolean) (ElapsedSeconds :type Float%20%28double-precision%29) (TriggeredSeconds :type Float%20%28double-precision%29) (InputAction :type Input%20Action%20Object%20Reference :default "/Game/ThirdPerson/Input/Actions/IA_pickup.IA_pickup"))
  (Default|CallGlassWall (stale EventBeginPlay _asbp_third_person_game_mode))
  (Variables|Default|Setdone true))

(event EventBeginPlay
  (bind _asbp_third_person_game_mode (Utilities|Casting|CastToBP_ThirdPersonGameMode (Game|GetGameMode))))

(fn ConstructionScript)