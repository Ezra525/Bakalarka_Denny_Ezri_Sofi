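; Puzzle actor that counts destroyed cables, Kabel1 and Kabel2, to remove itself once both are gone.
; Each cable's OnDestroyed increments KolkoKablovMam, then checks for two after a short delay.
; Only the Kabel1 branch calls DestroyActor; the Kabel2 branch calls SetLifeSpan with zero, which does not destroy the actor.
; Two timelines that would lower component R from its stored starting height are unconnected and never run.
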(event OnDestroyed(kabel2)
  (params (DestroyedActor :type Actor%20Object%20Reference))
  (Variables|Default|Setkolko%20kablov%20mam (+ 1 (Variables|Default|Getkolko%20kablov%20mam)))
  (Utilities|FlowControl|Delay 2.0)
  (if (== (Variables|Default|Getkolko%20kablov%20mam) 2)
    (Actor|SetLifeSpan 0.0)))

(event OnDestroyed(kabel1)
  (params (DestroyedActor :type Actor%20Object%20Reference))
  (Variables|Default|Setkolko%20kablov%20mam (+ 1 (Variables|Default|Getkolko%20kablov%20mam)))
  (Utilities|FlowControl|Delay 2.0)
  (if (== (Variables|Default|Getkolko%20kablov%20mam) 2)
    (Actor|DestroyActor)))

(event EventBeginPlay
  (Variables|Default|Setkolko%20kablov%20mam 0)
  (Variables|Default|SetRelative%20Location%20Z (.z (Variables|/Script/Engine.SceneComponent|GetRelativeLocation (Variables|Default|Getr)))))

(fn ConstructionScript)