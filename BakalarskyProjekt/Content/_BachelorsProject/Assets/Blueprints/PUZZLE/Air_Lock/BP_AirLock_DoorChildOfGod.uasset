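; Airlock puzzle door Blueprint that reacts to an AirlockSwitch event dispatcher.
; On BeginPlay it binds to the dispatcher, and when that fires it teleports the LeftSide component to an enormous relative X offset, removing it instantly rather than animating it.
; RightSide and the world-offset calculations are unused, and debug prints mark each step.
; The construction script only calls the parent's.
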(event Custom|AirlockSwitch_Event
  (Utilities|FlowControl|Sequence
    (:then_0
      (Transformation|SetRelativeLocation (Variables|Default|GetLeft_Side) "10000000000000000000.000000,0.000000,0.000000" false true)
      (Development|PrintString "done"))
    (:then_1
      (Development|PrintString "airlocok door here"))))

(event EventBeginPlay
  (EventDispatchers|AssignAirlockSwitch (delegate Custom|AirlockSwitch_Event))
  (Development|PrintString "it happend" true true "(R=1.000000,G=0.000000,B=0.057804,A=1.000000)"))

(fn ConstructionScript
  (|CallParentFunction))