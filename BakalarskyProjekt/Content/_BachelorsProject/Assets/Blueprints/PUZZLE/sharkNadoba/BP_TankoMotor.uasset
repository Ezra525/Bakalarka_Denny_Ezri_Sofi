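; BP_TankoMotor is a puzzle motor part that the player can pick up, which removes it from the world.
; Overlap events from PRINHA check whether the other actor is this motor, then toggle the motor's input and the SOMPRIKABLI flag.
; While the flag is set, the IA_pickup Enhanced Input action destroys the actor, with no inventory or notification logic in this Blueprint.
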(event OnActorBeginOverlap(PRINHA)
  (params (OverlappedActor :type Actor%20Object%20Reference) (OtherActor :type Actor%20Object%20Reference))
  (if (== OtherActor self)
    (Input|EnableInput (Game|GetPlayerController 0))
    (Variables|Default|SetSOM%20PRI%20KABLI true)))

(event OnActorEndOverlap(PRINHA)
  (params (OverlappedActor :type Actor%20Object%20Reference) (OtherActor :type Actor%20Object%20Reference))
  (if (== OtherActor self)
    (Input|DisableInput (Game|GetPlayerController 0))
    (Variables|Default|SetSOM%20PRI%20KABLI false)))

(event Input|EnhancedActionEvents|EnhancedInputActionIA_pickup
  (params (ActionValue :type Boolean) (ElapsedSeconds :type Float%20%28double-precision%29) (TriggeredSeconds :type Float%20%28double-precision%29) (InputAction :type Input%20Action%20Object%20Reference :default "/Game/ThirdPerson/Input/Actions/IA_pickup.IA_pickup"))
  (if (Variables|Default|GetSOM%20PRI%20KABLI)
    (Actor|DestroyActor)))

(fn ConstructionScript)