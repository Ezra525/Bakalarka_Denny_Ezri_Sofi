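; Puzzle lid (vrchnak) for the shark container, whose mesh is moved by damage events on its Koleso (wheel) component.
; Radial damage plays a timeline that increments the stored offset, which is seeded from relative Z but written to relative Y.
; Point damage plays a self-retriggering timeline that decrements it toward the start value until radial damage interrupts.
; A delayed Z-axis return chain is unconnected, and debug prints remain.
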(event OnTakeRadialDamage(koleso)
  (params (DamagedActor :type Actor%20Object%20Reference) (Damage :type Float%20%28single-precision%29) (DamageType :type Damage%20Type%20Object%20Reference) (Origin :type Vector :default "0, 0, 0") (HitInfo :type Hit%20Result%20Structure%20%28by%20ref%29) (InstigatedBy :type Controller%20Object%20Reference) (DamageCauser :type Actor%20Object%20Reference))
  (Variables|Default|Setteraz%20nie true)
  (Development|PrintString "damge kolesu")
  (bind _doorrotattion (Timeline|Timeline Play)
    (:Update
      (Transformation|SetRelativeLocation (Variables|Default|GetStaticMesh) (Math|Vector|MakeVector 0.0 (Math|Float|Lerp (Variables|Default|GetRelative%20Location%20Z) (+ (Variables|Default|GetRelative%20Location%20Z) 1.0) _doorrotattion) 0.0) false false)
      (Variables|Default|SetRelative%20Location%20Z (Math|Float|Lerp (Variables|Default|GetRelative%20Location%20Z) (+ (Variables|Default|GetRelative%20Location%20Z) 1.0) _doorrotattion)))))

(event OnTakePointDamage(koleso)
  (params (DamagedActor :type Actor%20Object%20Reference) (Damage :type Float%20%28single-precision%29) (InstigatedBy :type Controller%20Object%20Reference) (HitLocation :type Vector :default "0, 0, 0") (FHitComponent :type Primitive%20Component%20Object%20Reference) (BoneName :type Name :default "None") (ShotFromDirection :type Vector :default "0, 0, 0") (DamageType :type Damage%20Type%20Object%20Reference) (DamageCauser :type Actor%20Object%20Reference))
  (Variables|Default|Setteraz%20nie false)
  (Development|PrintString "mam ist dole")
  (if (not (>= (Variables|Default|Getstart%20location) (Variables|Default|GetRelative%20Location%20Z))) :!label _label
    (if (not (Variables|Default|Getteraz%20nie))
      (bind _doorrotattion (Timeline|Timeline_1 Play)
        (:Update
          (Development|PrintString "ideeeeeem  dole tiez" true true "(R=1.000000,G=0.000000,B=0.368924,A=1.000000)")
          (Transformation|SetRelativeLocation (Variables|Default|GetStaticMesh) (Math|Vector|MakeVector 0.0 (Math|Float|Lerp (Variables|Default|GetRelative%20Location%20Z) (- (Variables|Default|GetRelative%20Location%20Z) 0.5) _doorrotattion) 0.0) false false)
          (Variables|Default|SetRelative%20Location%20Z (Math|Float|Lerp (Variables|Default|GetRelative%20Location%20Z) (- (Variables|Default|GetRelative%20Location%20Z) 0.5) _doorrotattion))
          (goto _label))))))

(event EventBeginPlay
  (Variables|Default|SetRelative%20Location%20Z (.z (Variables|/Script/Engine.SceneComponent|GetRelativeLocation (Variables|Default|GetStaticMesh))))
  (Variables|Default|Setstart%20location (.z (Variables|/Script/Engine.SceneComponent|GetRelativeLocation (Variables|Default|GetStaticMesh)))))

(fn ConstructionScript)