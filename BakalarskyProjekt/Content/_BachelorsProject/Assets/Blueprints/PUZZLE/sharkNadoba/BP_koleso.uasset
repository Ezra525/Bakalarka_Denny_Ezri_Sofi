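; Puzzle wheel (koleso) in the shark puzzle that the Crab can turn once the wheel is powered by a hit on the Elektrika actor.
; Crab overlap enables the pickup input while powered, and leaving disables it.
; Triggered input plays a timeline that rolls the mesh forward, while releasing or canceling plays timelines that roll it back.
; Rotation updates also apply radial or point damage, and a delayed counter-based unwind loop is unconnected.
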(event OnActorHit(elektrika)
  (params (SelfActor :type Actor%20Object%20Reference) (OtherActor :type Actor%20Object%20Reference) (NormalImpulse :type Vector :default "0, 0, 0") (Hit :type Hit%20Result%20Structure%20%28by%20ref%29))
  ;[1 0.7799 0 0.5] Is powered?
  (Variables|Default|Setmam%20elekriku true))

(event OnActorBeginOverlap(Crab)
  (params (OverlappedActor :type Actor%20Object%20Reference) (OtherActor :type Actor%20Object%20Reference))
  ;[0 0.1382 0.15 0.5] Allow input
  (if (== OtherActor self)
    (if (Variables|Default|Getmam%20elekriku)
      (Input|EnableInput (Game|GetPlayerController 0))
      (Variables|Default|Setsom%20pri%20kolese true))))

(event OnActorEndOverlap(Crab)
  (params (OverlappedActor :type Actor%20Object%20Reference) (OtherActor :type Actor%20Object%20Reference))
  ;[0 0.1382 0.15 0.5] Allow input
  (if (== OtherActor self)
    (Input|DisableInput (Game|GetPlayerController 0))
    (Variables|Default|Setsom%20pri%20kolese false)))

(event Input|EnhancedActionEvents|EnhancedInputActionIA_pickup
  (params (ActionValue :type Boolean) (ElapsedSeconds :type Float%20%28double-precision%29) (TriggeredSeconds :type Float%20%28double-precision%29) (InputAction :type Input%20Action%20Object%20Reference :default "/Game/ThirdPerson/Input/Actions/IA_pickup.IA_pickup"))
  ;[0 0.1165 0.15 0.5] basically E interactions for crab
  (:Triggered
    (if (Variables|Default|Getsom%20pri%20kolese)
      (Variables|Default|Setrotationcounter (+ (Variables|Default|Getrotationcounter) 1))
      (bind _doorrotattion (Timeline|Timeline Play)
        (:Update
          (bind _output_get (Variables|Default|Setmine%20rotation (Math|Float|Lerp (Variables|Default|Getmine%20rotation) (+ (Variables|Default|Getmine%20rotation) 5.0) _doorrotattion)))
          (Transformation|SetRelativeRotation (Variables|Default|GetStaticMesh) (Math|Rotator|MakeRotator _output_get 0.0 0.0) false false)
          (Game|Damage|ApplyRadialDamage 1e+01 (Variables|Default|Getmy%20location) 1.0 0 0 0 0 false "ECC_Visibility")))))
  (:Canceled
    (bind _doorrotattion_2 (Timeline|Timeline_1 Play)
      (:Update
        (bind _output_get_2 (Variables|Default|Setmine%20rotation (Math|Float|Lerp (Variables|Default|Getmine%20rotation) (- (Variables|Default|Getmine%20rotation) 5.0) _doorrotattion_2)))
        (bind _sweephitresult (Transformation|SetRelativeRotation (Variables|Default|GetStaticMesh) (Math|Rotator|MakeRotator _output_get_2 0.0 0.0) true false))
        (Game|Damage|ApplyPointDamage self 1e+01 (Variables|Default|Getmy%20location) _sweephitresult))))
  (:Completed
    (bind _doorrotattion_3 (Timeline|Timeline_2 Play)
      (:Update
        (bind _output_get_3 (Variables|Default|Setmine%20rotation (Math|Float|Lerp (Variables|Default|Getmine%20rotation) (- (Variables|Default|Getmine%20rotation) 5.0) _doorrotattion_3)))
        (bind _sweephitresult_2 (Transformation|SetRelativeRotation (Variables|Default|GetStaticMesh) (Math|Rotator|MakeRotator _output_get_3 0.0 0.0) true false))
        (Game|Damage|ApplyPointDamage self 1e+01 (Variables|Default|Getmy%20location) _sweephitresult_2)))))

(event EventBeginPlay
  ;[0.005842 0.15 0 0.5] Set variables
  (Variables|Default|Setmy%20location (Transformation|GetActorLocation))
  (Variables|Default|Setmine%20rotation (.roll (Transformation|GetWorldRotation (Variables|Default|GetStaticMesh)))))

(fn ConstructionScript)