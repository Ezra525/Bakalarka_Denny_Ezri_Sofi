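; BP_electric is an electric hazard volume that deals periodic damage to actors with a HeathComponent.
; Box overlap stores the actor as the single target and, unless it is tagged "eel", damages it immediately and starts a looping one-second timer.
; The target is replaced before the tag check, and any qualifying actor leaving clears the timer.
; Each hit prints the damage result on screen for debugging.
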(event OnComponentBeginOverlap(Box)
  (params (OverlappedComponent :type Primitive%20Component%20Object%20Reference) (OtherActor :type Actor%20Object%20Reference) (OtherComp :type Primitive%20Component%20Object%20Reference) (OtherBodyIndex :type Integer) (bFromSweep :type Boolean) (SweepResult :type Hit%20Result%20Structure%20%28by%20ref%29))
  (Utilities|IsValid (Actor|GetComponentbyClass OtherActor "/Game/_BachelorsProject/Components/HeathComponent.HeathComponent_C")
    (:Is%20Valid
      (Variables|Default|SettargetCharaczer OtherActor)
      (if (not (Actor|ActorHasTag OtherActor "eel"))
        (Utilities|Time|SetTimerbyFunctionName 0 "ApplyDamage" 1.0 true)
        (CallFunction|ApplyDAmage)))))

(event OnComponentEndOverlap(Box)
  (params (OverlappedComponent :type Primitive%20Component%20Object%20Reference) (OtherActor :type Actor%20Object%20Reference) (OtherComp :type Primitive%20Component%20Object%20Reference) (OtherBodyIndex :type Integer))
  (Utilities|IsValid (Actor|GetComponentbyClass OtherActor "/Game/_BachelorsProject/Components/HeathComponent.HeathComponent_C")
    (:Is%20Valid
      (Utilities|Time|ClearTimerbyFunctionName 0 "ApplyDamage"))))

(fn ConstructionScript)

(fn ApplyDAmage
  (bind _returnvalue (Game|Damage|ApplyDamage (Variables|Default|GettargetCharaczer) 5e+01 0 0))
  (Development|PrintString (Utilities|String|ToString(Float) _returnvalue) true true "(R=0.028845,G=0.116165,B=1.000000,A=1.000000)" 1e+01))