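; Automatic swinging door that rotates its Doors component in yaw, driven by a Collision overlap.
; Begin overlap calls OpenDoor, playing a timeline swing, then after a long Delay a second, wider swing if EndOverlap is still false.
; End overlap plays a closing timeline after a short delay and sets EndOverlap, which is never reset here.
; Timelines use Play rather than PlayFromStart, with curves lerping the yaw.
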(event OnComponentBeginOverlap(collision)
  (params (OverlappedComponent :type Primitive%20Component%20Object%20Reference) (OtherActor :type Actor%20Object%20Reference) (OtherComp :type Primitive%20Component%20Object%20Reference) (OtherBodyIndex :type Integer) (bFromSweep :type Boolean) (SweepResult :type Hit%20Result%20Structure%20%28by%20ref%29))
  ;[0.15 0.15 0.15 0.5] Opendoor
  (CallFunction|OpenDoor))

(event OnComponentEndOverlap(collision)
  (params (OverlappedComponent :type Primitive%20Component%20Object%20Reference) (OtherActor :type Actor%20Object%20Reference) (OtherComp :type Primitive%20Component%20Object%20Reference) (OtherBodyIndex :type Integer))
  ;[0.15 0.15 0.15 0.5] closing
  (Utilities|FlowControl|Sequence
    (:then_0
      (if true
        (Utilities|FlowControl|Delay 2.0)
        (bind _doorrotattion (Timeline|Timeline_1 Play)
          (:Update
            (Transformation|SetRelativeRotation (Variables|Default|Getdoors) (Math|Rotator|MakeRotator 0.0 0.0 (Math|Float|Lerp 1.2e+02 0.0 _doorrotattion)) false false)))))
    (:then_1
      (Variables|Default|SetendOverlap true))))

(event Custom|OpenDoor
  ;[0.15 0.15 0.15 0.5] Opendoor
  (bind _doorrotattion (Timeline|Timeline Play)
    (:Update
      (Transformation|SetRelativeRotation (Variables|Default|Getdoors) (Math|Rotator|MakeRotator 0.0 0.0 (Math|Float|Lerp 6e+01 0.0 _doorrotattion)) false false)
      (Utilities|FlowControl|Delay 2e+01)
      (if (not (Variables|Default|GetendOverlap))
        (bind _doorrotattion_2 (Timeline|Timeline_0 Play)
          (:Update
            (Transformation|SetRelativeRotation (Variables|Default|Getdoors) (Math|Rotator|MakeRotator 0.0 0.0 (Math|Float|Lerp 0.0 1.2e+02 _doorrotattion_2)) false false)))))))

(fn ConstructionScript)