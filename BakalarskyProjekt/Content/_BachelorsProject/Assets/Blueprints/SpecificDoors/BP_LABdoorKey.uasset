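; BP_LABdoorKey is a key card pickup for a lab door that registers its CardID with the Brain_BP key ring.
; On BeginPlay it caches the first Brain_BP actor in the level.
; A trigger overlap adds CardID for any actor, then destroys the pickup only if that actor is BP_ThirdPersonCharacter.
; It also looks up BP_LABdoor1 but leaves the result unused.
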(event OnComponentBeginOverlap(Trigger)
  (params (OverlappedComponent :type Primitive%20Component%20Object%20Reference) (OtherActor :type Actor%20Object%20Reference) (OtherComp :type Primitive%20Component%20Object%20Reference) (OtherBodyIndex :type Integer) (bFromSweep :type Boolean) (SweepResult :type Hit%20Result%20Structure%20%28by%20ref%29))
  ;[0.15 0.15 0.15 0.5] zobratie kluca
  (Default|AddtoKeyRing (Variables|Default|GetBrainRef) (Variables|Default|GetCardID))
  (Utilities|Casting|CastToBP_ThirdPersonCharacter OtherActor)
  (Actor|GetActorOfClass "/Game/_BachelorsProject/Assets/Blueprints/SpecificDoors/BP_LABdoor1.BP_LABdoor1_C")
  (Actor|DestroyActor))

(event Custom|GetBrainRef
  ;[0.15 0.15 0.15 0.5] Brain prepojenie Dvery a Cards
  (bind _outactors (Actor|GetAllActorsOfClass "/Game/_BachelorsProject/Assets/Blueprints/SpecificDoors/Brain_BP.Brain_BP_C"))
  (Variables|Default|SetBrainRef (Utilities|Array|Get(acopy) _outactors)))

(event EventBeginPlay
  ;[0.15 0.15 0.15 0.5] Brain prepojenie Dvery a Cards
  (CallFunction|GetBrainRef))

(fn ConstructionScript)