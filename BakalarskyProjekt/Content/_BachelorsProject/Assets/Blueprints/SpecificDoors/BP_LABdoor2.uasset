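; BP_LABdoor2 is a lab door that opens only when the player's card ring holds the card matching its CardID.
; On BeginPlay it caches the Brain_BP actor, which holds the CardRing.
; Each successful OPenDoorCheck increments a collected counter, and reaching the maximum triggers OpenDoor once through a DoOnce.
; OpenDoor plays a timeline that swings the door's yaw open, while CollectItem is an empty event.
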(event Custom|OpenDoor
  ;[0.15 0.15 0.15 0.5] animacia otvorenia
  (bind _doorrotattion (Timeline|OpenDoorAnim Play)
    (:Update
      (Transformation|SetRelativeRotation (Variables|Default|Getdoor) (Math|Rotator|MakeRotator 0.0 0.0 (Math|Float|Lerp 0.0 1.2e+02 _doorrotattion)) false false))))

(event Custom|GetBrainRef
  ;[0.15 0.15 0.15 0.5] Brain prepojenie kariet a dveri
  (bind _outactors (Actor|GetAllActorsOfClass "/Game/_BachelorsProject/Assets/Blueprints/SpecificDoors/Brain_BP.Brain_BP_C"))
  (Variables|Default|SetBrainRef (Utilities|Array|Get(acopy) _outactors)))

(event Custom|OPenDoorCheck
  ;[0.15 0.15 0.15 0.5] Mas spravny kluc?
  (if (Utilities|Array|ContainsItem (Variables|/Game/_BachelorsProject/Assets/Blueprints/SpecificDoors/Brain_BP.Brain_BP_C|GetCardRing (Variables|Default|GetBrainRef)) (Variables|Default|GetCardID))
    (Math|Integer|IncrementInt (Variables|Default|GetCurrentItemsCollected)
      (:%20%20
        (if (>= (Variables|Default|GetCurrentItemsCollected) (Variables|Default|GetMaxItemsCollected))
          (Utilities|FlowControl|DoOnce false
            (:Completed
              (CallFunction|OpenDoor))))))))

(event Custom|CollectItem
  ;[0.15 0.15 0.15 0.5] animacia otvorenia
)

(event EventBeginPlay
  ;[0.15 0.15 0.15 0.5] Brain prepojenie kariet a dveri
  (CallFunction|GetBrainRef))

(fn ConstructionScript)