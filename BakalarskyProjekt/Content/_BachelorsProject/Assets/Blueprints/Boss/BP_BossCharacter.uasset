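; Flying boss character that roams to random reachable points within a radius of itself and hunts the player on sight.
; Pawn sensing raises fly speed and starts an AI move to the player, while a retriggerable delay restores slow roaming once sightings stop.
; Reaching the player plays a fly-attack montage and damages a player with a health component, using DoOnce and the montage length as cooldown.
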(event OnSeePawn(PawnSensing)
  (params (Pawn :type Pawn%20Object%20Reference))
  ;[0.15 0.15 0.15 0.5] chase player
  (Variables|Default|SetCanAttack true)
  (Utilities|FlowControl|Sequence
    (:then_0
      (Variables|/Script/Engine.CharacterMovementComponent|SetMaxFlySpeed (Variables|Character|GetCharacterMovement) 2e+02)
      (AI|AIMoveTo self "0, 0, 0" (Game|GetPlayerCharacter 0) 8e+01 false
        (:OnSuccess
          (if (Variables|Default|GetCanAttack)
            (Variables|Default|SetCanAttack false)
            (CallFunction|Attack)))))
    (:then_1
      (Utilities|FlowControl|RetriggerableDelay 1.0)
      (CallFunction|BossRoam)
      (Variables|/Script/Engine.CharacterMovementComponent|SetMaxFlySpeed (Variables|Character|GetCharacterMovement) 8e+01))))

(event Custom|bossRoam
  ;[0.15 0.15 0.15 0.5] Roaming
  (AI|AIMoveTo self (.RandomLocation (AI|Navigation|GetRandomReachablePointinRadius (Transformation|GetActorLocation) 1.5e+03 0 0)) 0 5.0 false
    (:OnSuccess
      (CallFunction|BossRoam))
    (:OnFail
      (CallFunction|BossRoam))))

(event Custom|attack
  (bind _returnvalue (Game|GetPlayerCharacter 0))
  ;[0.15 0.15 0.15 0.5] attack
  (Utilities|FlowControl|DoOnce false :!label _label
    (:Completed
      (bind _returnvalue_2 (Animation|PlayAnimMontage "/Game/Fab/FourEvilDragonsPBR/Animations/DragonTheSoulEater/FlyAttackAnim_Montage.FlyAttackAnim_Montage" 1.0 "None"))
      (Utilities|IsValid (Actor|GetComponentbyClass _returnvalue "/Game/_BachelorsProject/Components/HeathComponent.HeathComponent_C")
        (:Is%20Valid
          (bind _returnvalue_3 (Game|Damage|ApplyDamage _returnvalue 1e+01 0 0))
          (Development|PrintString (Utilities|String|ToString(Float) _returnvalue_3) true true "(R=1.000000,G=0.782915,B=0.000000,A=1.000000)" 1e+01)
          (Utilities|FlowControl|Delay _returnvalue_2)
          (Variables|Default|SetCanAttack true)
          (goto _label Reset))))))

(event EventBeginPlay
  ;[0.15 0.15 0.15 0.5] setup
  (Collision|SetCollisionResponsetoChannel (Variables|Character|GetMesh) "ECC_Camera" "ECR_Ignore")
  (CallFunction|BossRoam))

(fn ConstructionScript)