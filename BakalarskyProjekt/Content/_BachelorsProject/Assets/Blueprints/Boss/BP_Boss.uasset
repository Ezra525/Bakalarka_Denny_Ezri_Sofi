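; Boss actor Blueprint with small query functions for climbing detection, possession and identity.
; ClimbingLineTrace fires a debug-drawn visibility trace a short distance forward from the actor and returns the hit.
; Two getters expose a stored possession duration and the boss's name, converted to a Name.
; The construction script is empty and no event logic is present.
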(fn ConstructionScript)

(fn ClimbingLineTrace
  (bind _returnvalue (Transformation|GetActorLocation))
  (bind (_outhit _returnvalue_2) (Collision|LineTraceByChannel _returnvalue (+ _returnvalue (* (Math|Vector|GetForwardVector (Transformation|GetActorRotation)) 1e+02)) "TraceTypeQuery1" false 0 "ForDuration"))
  (return _outhit _returnvalue_2))

(fn GetPossesionduration
  (return (Variables|Default|GetpossesionTime_0)))

(fn MyNameIs
  (return (Utilities|String|StringToName (Variables|Default|GetI%20have%20name%20bitch!))))