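; BP_collectItem is a collectible that the player picks up by pressing the pickup input while in range.
; Box overlaps with BP_crabcollision enable and disable the actor's input for the first player controller, so the action only responds nearby.
; On pickup, it decrements the Remaining count on BP_ThirdPersonGameMode, adds a new W_itemsCollected widget to the viewport and destroys itself.
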(event OnComponentBeginOverlap(Box)
  (params (OverlappedComponent :type Primitive%20Component%20Object%20Reference) (OtherActor :type Actor%20Object%20Reference) (OtherComp :type Primitive%20Component%20Object%20Reference) (OtherBodyIndex :type Integer) (bFromSweep :type Boolean) (SweepResult :type Hit%20Result%20Structure%20%28by%20ref%29))
  (Utilities|Casting|CastToBP_crabcollision OtherActor)
  (Input|EnableInput (Game|GetPlayerController 0)))

(event OnComponentEndOverlap(Box)
  (params (OverlappedComponent :type Primitive%20Component%20Object%20Reference) (OtherActor :type Actor%20Object%20Reference) (OtherComp :type Primitive%20Component%20Object%20Reference) (OtherBodyIndex :type Integer))
  (Utilities|Casting|CastToBP_crabcollision OtherActor)
  (Input|DisableInput (Game|GetPlayerController 0)))

(event Input|EnhancedActionEvents|EnhancedInputActionIA_pickup
  (params (ActionValue :type Boolean) (ElapsedSeconds :type Float%20%28double-precision%29) (TriggeredSeconds :type Float%20%28double-precision%29) (InputAction :type Input%20Action%20Object%20Reference :default "/Game/ThirdPerson/Input/Actions/IA_pickup.IA_pickup"))
  (:Started
    (bind _asbp_third_person_game_mode (Utilities|Casting|CastToBP_ThirdPersonGameMode (Game|GetGameMode)))
    (bind _result (Math|Integer|DecrementInt (Variables|/Game/ThirdPerson/Blueprints/BP_ThirdPersonGameMode.BP_ThirdPersonGameMode_C|Getremaining _asbp_third_person_game_mode))
      (:%20%20
        (Variables|/Game/ThirdPerson/Blueprints/BP_ThirdPersonGameMode.BP_ThirdPersonGameMode_C|Setremaining _asbp_third_person_game_mode _result)
        (bind _returnvalue (UserInterface|CreateWidget "/Game/_BachelorsProject/Assets/Blueprints/collectibles/W_itemsCollected.W_itemsCollected_C"))
        (UserInterface|Viewport|AddtoViewport _returnvalue 0)
        (Actor|DestroyActor)))))

(fn ConstructionScript)