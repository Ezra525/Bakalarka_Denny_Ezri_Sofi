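; BP_CameraRail is an unfinished camera rail actor with a spline and a cine camera, where every event and the construction script is empty.
; Disconnected nodes sketch finding the spline distance closest to a player location, moving the camera, setting look-at tracking on the player pawn and switching the view target to itself.
; None of this logic is wired, so MoveCameraonRails currently does nothing.
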(event EventBeginPlay)

(event Collision|EventActorBeginOverlap
  (params (OtherActor :type Actor%20Object%20Reference)))

(event EventTick
  (params (DeltaSeconds :type Float%20%28single-precision%29)))

(event EventMoveCameraonRails
  (params (Rail%20ID :type Name :default "None") (Player%20Location :type Vector :default "0, 0, 0")))

(fn ConstructionScript)