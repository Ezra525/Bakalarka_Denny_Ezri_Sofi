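; BP_tabletnotes is a pickup note item actor whose mesh is set from its ItemModel variable in the construction script.
; Its Interactitem function prints a pickup message and returns the ItemModel mesh to the caller.
; A Destroyitem event removes the actor after a short delay, but the call to it inside Interactitem is disconnected, so interacting leaves the item in place.
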(event Custom|Destroy%20item
  (Utilities|FlowControl|Delay 0.2)
  (Actor|DestroyActor))

(fn ConstructionScript
  (Components|StaticMesh|SetStaticMesh (Variables|Default|GetStaticMesh) (Variables|Default|GetItemModel)))

(fn Interactitem
  (Development|PrintString "item picked up")
  (return (Variables|Default|GetItemModel)))