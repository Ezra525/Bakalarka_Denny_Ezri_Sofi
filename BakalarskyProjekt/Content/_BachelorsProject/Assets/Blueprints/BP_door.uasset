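; BP_door is a door that swings open once enough items have been collected.
; OPenDoorCheck increments a collected count and, once it reaches the maximum, fires OpenDoor through a DoOnce so it only runs once.
; OpenDoor plays a timeline that lerps the Door component's relative yaw from closed to open.
; The CollectItem event is empty.
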(event Custom|OpenDoor
  (bind _doorrotattion (Timeline|OpenDoorAnim Play)
    (:Update
      (Transformation|SetRelativeRotation (Variables|Default|Getdoor) (Math|Rotator|MakeRotator 0.0 0.0 (Math|Float|Lerp 0.0 1.2e+02 _doorrotattion)) false false))))

(event Custom|OPenDoorCheck
  (Math|Integer|IncrementInt (Variables|Default|GetCurrentItemsCollected)
    (:%20%20
      (if (>= (Variables|Default|GetCurrentItemsCollected) (Variables|Default|GetMaxItemsCollected))
        (Utilities|FlowControl|DoOnce false
          (:Completed
            (CallFunction|OpenDoor)))))))

(event Custom|CollectItem)

(fn ConstructionScript)