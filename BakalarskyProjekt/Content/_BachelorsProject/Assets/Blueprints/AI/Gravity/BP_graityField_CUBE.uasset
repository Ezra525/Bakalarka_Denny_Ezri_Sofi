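; Cube variant of a gravity field that overrides GetGravityDirection to supply a pull direction for a given actor.
; It returns the unit vector from the actor toward a point built from the field's colliding bounds origin plus the clamped per-axis offset.
; Both clamp limits equal the positive box extent, so the target always resolves to the bounds' positive corner.
; The event graph holds only disabled default events.
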(event EventBeginPlay
  (|CallParentFunction) ; This node is disabled and will not be called.\nDrag off pins to build functionality.
)

(event Collision|EventActorBeginOverlap
  (params (OtherActor :type Actor%20Object%20Reference))
  (|CallParentFunction OtherActor) ; This node is disabled and will not be called.\nDrag off pins to build functionality.
)

(event EventTick
  (params (DeltaSeconds :type Float%20%28single-precision%29))
  (|CallParentFunction DeltaSeconds) ; This node is disabled and will not be called.\nDrag off pins to build functionality.
)

(fn ConstructionScript
  (|CallParentFunction))

(fn GetGravityDirection
  (params (actor :type Actor%20Object%20Reference))
  (bind _returnvalue (Transformation|GetActorLocation actor))
  (bind _self self)
  (bind (_origin _boxextent) (Collision|GetActorBounds _self true true))
  (bind _returnvalue_2 (- _origin _returnvalue))
  (|CallParentFunction actor)
  (return (Math|Vector|GetUnitDirection(Vector) _returnvalue (+ _origin (Math|Vector|MakeVector (Math|Float|Clamp(Float) (.x _returnvalue_2) (.x _boxextent) (.x _boxextent)) (Math|Float|Clamp(Float) (.y _returnvalue_2) (.y _boxextent) (.y _boxextent)) (Math|Float|Clamp(Float) (.z _returnvalue_2) (.z _boxextent) (.z _boxextent)))))))