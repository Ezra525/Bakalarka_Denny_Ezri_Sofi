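; Test actor for crab walking that orients itself to the surface beneath it, moved by forward and right events along its own axes.
; The right event runs on into the forward movement step, which records per-move displacement as velocity.
; Each Tick traces along local down, skewed by that velocity to look ahead, then sets rotation from the hit normal and current forward, without checking for a hit.
; Debug drawing shows the trace and normal-change axis.
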(event Custom|forward
  (params (NewParam :type Float%20%28double-precision%29))
  (bind _returnvalue (Transformation|GetActorLocation))
  (Transformation|SetActorLocation (+ _returnvalue (* (Transformation|GetActorForwardVector) (Utilities|Time|GetWorldDeltaSeconds) (stale Custom|right NewParam) (Math|Float|MakeLiteralFloat 2e+02))) false false)
  (Variables|Default|SetvelocityChar (- _returnvalue (Variables|Default|GetprevLocation))))

(event Custom|right
  (params (NewParam :type Float%20%28double-precision%29))
  (bind _returnvalue (Transformation|GetActorLocation))
  (bind _returnvalue_2 (Utilities|Time|GetWorldDeltaSeconds))
  (bind _returnvalue_3 (Math|Float|MakeLiteralFloat 2e+02))
  (Transformation|SetActorLocation (+ _returnvalue (* (Transformation|GetActorRightVector) (stale Custom|forward NewParam) _returnvalue_2 _returnvalue_3)) false false)
  (Transformation|SetActorLocation (+ _returnvalue (* (Transformation|GetActorForwardVector) _returnvalue_2 NewParam _returnvalue_3)) false false)
  (Variables|Default|SetvelocityChar (- _returnvalue (Variables|Default|GetprevLocation))))

(event EventBeginPlay)

(event Collision|EventActorBeginOverlap
  (params (OtherActor :type Actor%20Object%20Reference)))

(event EventTick
  (params (DeltaSeconds :type Float%20%28single-precision%29))
  (bind _linetracestart (Variables|Default|GetlineTraceStart))
  (bind _returnvalue (Transformation|GetWorldLocation _linetracestart))
  (Utilities|FlowControl|Sequence
    (:then_0
      (Variables|Default|SetprevLocation (Transformation|GetActorLocation)))
    (:then_1
      (bind _outhit (Collision|LineTraceByChannel _returnvalue (+ _returnvalue (* (* (Transformation|GetActorUpVector) -1.0) 8e+01) (* (Variables|Default|GetvelocityChar) 12.0)) "TraceTypeQuery1" true 0 "ForDuration"))
      (Rendering|Debug|DrawDebugLine (.Location (Collision|BreakHitResult _outhit)) (+ (.Location (Collision|BreakHitResult _outhit)) (* (Math|Vector|Normalize (Math|Vector|CrossProduct (Variables|Default|GetoldNormal) (.Normal (Collision|BreakHitResult _outhit)))) 7e+01)) "(R=0.998476,G=0.351400,B=1.000000,A=1.000000)" 0.2 3.0)
      (Transformation|SetActorRotation (Math|Rotator|MakeRotfromZX (.Normal (Collision|BreakHitResult _outhit)) (Transformation|GetActorForwardVector)))
      (if (not (Utilities|Operators|EqualEqual (.Normal (Collision|BreakHitResult _outhit)) (Variables|Default|GetoldNormal) 1e-05))
        (Variables|Default|SetoldNormal (.Normal (Collision|BreakHitResult _outhit)))))))

(fn ConstructionScript)