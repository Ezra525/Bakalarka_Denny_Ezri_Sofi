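; Test fish pawn that the player can possess, with health, damage feedback and respawning.
; Damage feeds the health component; when that returns true, the player controller repossesses the game mode's original pawn and the fish hides.
; Each hit shows a post-process effect, faded by timeline after a delay.
; The game mode's player-death event restores its start location, visibility and health; helper functions provide a forward trace, possession duration and placeholder name.
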(event Custom|CustomEvent
  ;[0.6376 0 0.04374 0.502] Respawn
  (Transformation|SetActorLocation (stale EventBeginPlay _returnvalue) false false)
  (Rendering|SetActorHiddenInGame false)
  (Variables|/Game/_BachelorsProject/Components/HeathComponent.HeathComponent_C|SetCurrentHealth (Variables|Default|GetHeathComponent) 100))

(event EventBeginPlay
  ;[0.6376 0 0.04374 0.502] Respawn
  (Variables|Default|Setpossess false)
  (bind _returnvalue (Transformation|GetActorLocation))
  (bind _asbp_third_person_game_mode (Utilities|Casting|CastToBP_ThirdPersonGameMode (Game|GetGameMode)))
  (EventDispatchers|BindEventtoOnPlayerDeath _asbp_third_person_game_mode (delegate Custom|CustomEvent)))

(event Game|Damage|EventAnyDamage
  (params (Damage :type Float%20%28single-precision%29) (DamageType :type Damage%20Type%20Object%20Reference) (InstigatedBy :type Controller%20Object%20Reference) (DamageCauser :type Actor%20Object%20Reference))
  (bind _damagepostproces (Variables|Default|Getdamagepostproces))
  ;[0.6376 0 0.04374 0.502] Dammage
  (Utilities|FlowControl|Sequence
    (:then_0
      (bind _sheathdepleted (Default|Takedamage (Variables|Default|GetHeathComponent) (Math|Float|Truncate Damage)))
      (if _sheathdepleted
        (bind _asbp_third_person_game_mode (Utilities|Casting|CastToBP_ThirdPersonGameMode (Game|GetGameMode)))
        (Pawn|UnPossess (Game|GetPlayerController 0))
        (Pawn|Possess (Game|GetPlayerController 0) (Variables|/Game/ThirdPerson/Blueprints/BP_ThirdPersonGameMode.BP_ThirdPersonGameMode_C|GetOriginalTypek _asbp_third_person_game_mode))
        (Rendering|SetActorHiddenInGame self true)))
    (:then_1
      (Variables|/Script/Engine.PostProcessComponent|SetBlendWeight _damagepostproces 1.0)
      (Utilities|FlowControl|Delay 3.0)
      (bind _fadeout (Timeline|Timeline PlayFromStart)
        (:Update
          (Variables|/Script/Engine.PostProcessComponent|SetBlendWeight _damagepostproces _fadeout))))))

(event EventPossessed
  (params (NewController :type Controller%20Object%20Reference))
  ;[0.15 0.15 0.15 0.5] Ked unpossest  je ai
  (Variables|Default|Setpossess true))

(event EventUnpossessed
  (params (OldController :type Controller%20Object%20Reference))
  ;[0.15 0.15 0.15 0.5] Ked unpossest  je ai
  (Utilities|FlowControl|Sequence
    (:then_1
      (Variables|Default|Setpossess false))))

(fn ConstructionScript)

(fn ClimbingLineTrace
  (bind _returnvalue (Transformation|GetActorLocation))
  (bind (_outhit _returnvalue_2) (Collision|LineTraceByChannel _returnvalue (+ _returnvalue (* (Math|Vector|GetForwardVector (Transformation|GetActorRotation)) 1e+02)) "TraceTypeQuery1" false 0 "ForDuration"))
  (return _outhit _returnvalue_2))

(fn GetPossesionduration
  (return (Variables|Default|GetpossesionTime_0)))

(fn MyNameIs
  (return "None"))