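; Possessable shark that reverts to its default AI controller when unpossessed and can break through walls.
; Damage goes to its health component; when that returns true, the player re-possesses the game mode's original character and the shark is hidden.
; Its nose collider spawns an active field-system master field at overlapped "Wall"-tagged actors and destroys it when the overlap ends.
; It also reports its possession duration through a getter.
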(event OnComponentBeginOverlap(SharkNose)
  (params (OverlappedComponent :type Primitive%20Component%20Object%20Reference) (OtherActor :type Actor%20Object%20Reference) (OtherComp :type Primitive%20Component%20Object%20Reference) (OtherBodyIndex :type Integer) (bFromSweep :type Boolean) (SweepResult :type Hit%20Result%20Structure%20%28by%20ref%29))
  (if (Actor|ActorHasTag OtherActor "Wall")
    (Utilities|FlowControl|DoOnce false :!label _label
      (:Completed
        (bind _returnvalue (Game|SpawnActorfromClass "/Engine/EditorResources/FieldNodes/FS_MasterField.FS_MasterField_C" (Math|Transform|MakeTransform (Transformation|GetActorLocation OtherActor) "0, 0, 0" "1.000000,1.000000,1.000000") "AlwaysSpawn" "MultiplyWithRoot" 0 0))
        (Variables|/Engine/EditorResources/FieldNodes/FS_MasterField.FS_MasterField_C|SetActivationType _returnvalue "NewEnumerator2")
        (Variables|/Engine/EditorResources/FieldNodes/FS_MasterField.FS_MasterField_C|SetField%20Active _returnvalue true)
        (goto _label Reset)))))

(event OnComponentEndOverlap(SharkNose)
  (params (OverlappedComponent :type Primitive%20Component%20Object%20Reference) (OtherActor :type Actor%20Object%20Reference) (OtherComp :type Primitive%20Component%20Object%20Reference) (OtherBodyIndex :type Integer))
  (if (Actor|ActorHasTag OtherActor "Wall")
    (Actor|DestroyActor (stale OnComponentBeginOverlap(SharkNose) _returnvalue))))

(event Game|Damage|EventAnyDamage
  (params (Damage :type Float%20%28single-precision%29) (DamageType :type Damage%20Type%20Object%20Reference) (InstigatedBy :type Controller%20Object%20Reference) (DamageCauser :type Actor%20Object%20Reference))
  (bind _sheathdepleted (Default|Takedamage (Variables|Default|GetHeathComponent) (Math|Float|Truncate Damage)))
  (if _sheathdepleted
    (bind _asbp_third_person_game_mode (Utilities|Casting|CastToBP_ThirdPersonGameMode (Game|GetGameMode)))
    (Pawn|UnPossess (Game|GetPlayerController 0))
    (Pawn|Possess (Game|GetPlayerController 0) (Variables|/Game/ThirdPerson/Blueprints/BP_ThirdPersonGameMode.BP_ThirdPersonGameMode_C|GetOriginalTypek _asbp_third_person_game_mode))
    (Rendering|SetActorHiddenInGame self true)))

(event EventUnpossessed
  (params (OldController :type Controller%20Object%20Reference))
  ;[0.15 0.15 0.15 0.5] Ked unpossest  je ai
  (Pawn|SpawnDefaultController))

(fn ConstructionScript)

(fn GetPossesionduration
  (return (Variables|Default|GetpossesionTime_0)))