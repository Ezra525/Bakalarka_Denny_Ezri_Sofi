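; Test fish AI that flies with Flying movement mode, wandering until AI Perception reports a Player-tagged actor, then chasing it.
; Looping timers poll perception and steer by look-at movement input.
; Wander points come from random line traces ending relative to world origin; a sphere trace finding an Enemy-tagged pawn there triggers repicking.
; A forward sphere trace hitting the player only prints "Attack", pauses, then resumes.
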(event Custom|Detect%20Player
  (for _array_element (Class|AIPerceptionComponent|GetKnownPerceivedActors (Variables|Default|GetAIPerception))
    (if (Actor|ActorHasTag _array_element "Player")
      (Variables|Default|SetTarget _array_element))))

(event Custom|Fly%20To%20Random%20Location
  (bind _returnvalue (Transformation|GetActorLocation))
  (bind _location (Variables|Default|GetLocation))
  (bind _location_2 (Variables|Default|GetLocation))
  (bind _returnvalue_2 (Math|Rotator|FindLookatRotation _returnvalue _location_2))
  (Variables|Default|GetTarget
    (:then
      (Utilities|Time|ClearandInvalidateTimerbyHandle (stale Custom|Move%20To _returnvalue_3))
      (Utilities|Time|SetTimerbyEvent (delegate Custom|Move%20To) 0.1 :!label _label)
      (Pawn|Components|CharacterMovement|SetMovementMode (Variables|Character|GetCharacterMovement) "MOVE_Flying" 0))
    (:else
      (bind (_outhit _returnvalue_3) (Collision|SphereTraceForObjects _location _location 1e+02 (Utilities|Array|MakeArray "ObjectTypeQuery3") false 0 "Persistent" false))
      (Pawn|Input|AddMovementInput (Math|Vector|GetForwardVector (Math|Rotator|MakeRotator 0.0 (.pitch _returnvalue_2) (.yaw _returnvalue_2))) 1.0 false)
      (if _returnvalue_3
        (if (Actor|ActorHasTag (.HitActor (Collision|BreakHitResult _outhit)) "Enemy")
          (Utilities|Time|ClearandInvalidateTimerbyHandle (stale Custom|Move%20To _returnvalue_3))
          (Utilities|FlowControl|RetriggerableDelay 0.2)
          (goto _label))))))

(event Custom|Move%20To
  (Variables|Default|GetTarget
    (:then
      (bind _returnvalue (Utilities|Time|SetTimerbyEvent (delegate Custom|Fly%20To%20Player) 0.01 true)))
    (:else
      (bind (_outhit _returnvalue_2) (Collision|LineTraceForObjects (Transformation|GetActorLocation) (* (+ (* (Transformation|GetActorForwardVector) (Math|Random|RandomIntegerinRange -1 1)) (* (Transformation|GetActorRightVector) (Math|Random|RandomIntegerinRange -1 1)) (* (Transformation|GetActorUpVector) (Math|Random|RandomIntegerinRange -1 1))) (Math|Random|RandomFloatinRange 2e+03 6e+03)) (Utilities|Array|MakeArray "ObjectTypeQuery1" "ObjectTypeQuery2" "ObjectTypeQuery4" "ObjectTypeQuery3" "ObjectTypeQuery5" "ObjectTypeQuery6") false 0 "ForDuration"))
      (if true
        (Variables|Default|SetLocation (select _returnvalue_2 (.ImpactPoint (Collision|BreakHitResult _outhit)) (.TraceEnd (Collision|BreakHitResult _outhit))))
        (bind _returnvalue_3 (Utilities|Time|SetTimerbyEvent (delegate Custom|Fly%20To%20Random%20Location) 0.01 true))
        (else
          (Development|PrintString "no Path avaiilable"))))))

(event Custom|Fly%20To%20Player
  (bind _returnvalue (Transformation|GetActorLocation))
  (bind _returnvalue_2 (Transformation|GetActorLocation))
  (bind _target (Variables|Default|GetTarget))
  (bind _returnvalue_3 (Transformation|GetActorLocation _target))
  (bind _returnvalue_4 (Math|Rotator|FindLookatRotation _returnvalue_2 _returnvalue_3))
  (bind (_outhit _returnvalue_5) (Collision|SphereTraceForObjects _returnvalue (+ _returnvalue (* (Transformation|GetActorForwardVector) 1e+02)) 1e+02 (Utilities|Array|MakeArray "ObjectTypeQuery3") false 0 "ForDuration"))
  (if _returnvalue_5
    (if (Actor|ActorHasTag (.HitActor (Collision|BreakHitResult _outhit)) "Player")
      (Development|PrintString "Attack")
      (Utilities|Time|ClearandInvalidateTimerbyHandle (stale Custom|Move%20To _returnvalue))
      (Utilities|FlowControl|RetriggerableDelay 1.0)
      (Utilities|Time|SetTimerbyEvent (delegate Custom|Move%20To) 0.1)
      (Pawn|Components|CharacterMovement|SetMovementMode (Variables|Character|GetCharacterMovement) "MOVE_Flying" 0)
      (else
        (Pawn|Input|AddMovementInput (Math|Vector|GetForwardVector (Math|Rotator|MakeRotator 0.0 (.pitch _returnvalue_4) (.yaw _returnvalue_4))) 1e+02 false :!label _label)))
    (else
      (goto _label))))

(event EventBeginPlay
  (Utilities|Time|SetTimerbyEvent (delegate Custom|Detect%20Player) 0.1 true)
  (Utilities|Time|SetTimerbyEvent (delegate Custom|Move%20To) 0.1)
  (Pawn|Components|CharacterMovement|SetMovementMode (Variables|Character|GetCharacterMovement) "MOVE_Flying" 0))

(fn ConstructionScript)

(fn ClimbingLineTrace
  (bind _returnvalue (Transformation|GetActorLocation))
  (bind (_outhit _returnvalue_2) (Collision|LineTraceByChannel _returnvalue (+ _returnvalue (* (Math|Vector|GetForwardVector (Transformation|GetActorRotation)) 1e+02)) "TraceTypeQuery1" false 0 "ForDuration"))
  (return _outhit _returnvalue_2))

(fn GetPossesionduration
  (return (Variables|Default|GetpossesionTime_0)))

(fn MyNameIs
  (return "None"))