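; BP_eel is a possessable eel pawn that returns to AI control through its default controller when unpossessed.
; When HeathComponent's damage call returns true, player control passes back to the game mode's OriginalTypek and the eel is hidden.
; It saves its start location and, on the game mode's player-death event, respawns there visible with restored health.
; Helper functions provide a forward climbing trace and the possession duration.
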(event Custom|CustomEvent
  ;[0.009721 0.006049 0.15 0.502] Respawn
  (Transformation|SetActorLocation (stale EventBeginPlay _returnvalue) false false)
  (Rendering|SetActorHiddenInGame false)
  (Variables|/Game/_BachelorsProject/Components/HeathComponent.HeathComponent_C|SetCurrentHealth (Variables|Default|GetHeathComponent) 100))

(event EventBeginPlay
  ;[0.009721 0.006049 0.15 0.502] Respawn
  (bind _returnvalue (Transformation|GetActorLocation))
  (bind _asbp_third_person_game_mode (Utilities|Casting|CastToBP_ThirdPersonGameMode (Game|GetGameMode)))
  (EventDispatchers|BindEventtoOnPlayerDeath _asbp_third_person_game_mode (delegate Custom|CustomEvent)))

(event Game|Damage|EventAnyDamage
  (params (Damage :type Float%20%28single-precision%29) (DamageType :type Damage%20Type%20Object%20Reference) (InstigatedBy :type Controller%20Object%20Reference) (DamageCauser :type Actor%20Object%20Reference))
  (bind _sheathdepleted (Default|Takedamage (Variables|Default|GetHeathComponent) (Math|Float|Truncate Damage)))
  (if _sheathdepleted
    (bind _asbp_third_person_game_mode (Utilities|Casting|CastToBP_ThirdPersonGameMode (Game|GetGameMode)))
    (Pawn|UnPossess (Game|GetPlayerController 0))
    (Pawn|Possess (Game|GetPlayerController 0) (Variables|/Game/ThirdPerson/Blueprints/BP_ThirdPersonGameMode.BP_ThirdPersonGameMode_C|GetOriginalTypek _asbp_third_person_game_mode))
    (Rendering|SetActorHiddenInGame self true)))

(event EventUnpossessed
  (params (OldController :type Controller%20Object%20Reference))
  ;[0.15 0.15 0.15 0.5] Ked unpossest  je ai
  (Pawn|SpawnDefaultController))

(fn ConstructionScript)

(fn ClimbingLineTrace
  (bind _returnvalue (Transformation|GetActorLocation))
  (bind (_outhit _returnvalue_2) (Collision|LineTraceByChannel _returnvalue (+ _returnvalue (* (Math|Vector|GetForwardVector (Transformation|GetActorRotation)) 1e+02)) "TraceTypeQuery1" false 0 "ForDuration"))
  (return _outhit _returnvalue_2))

(fn GetPossesionduration
  (return (Variables|Default|GetpossesionTime_0)))