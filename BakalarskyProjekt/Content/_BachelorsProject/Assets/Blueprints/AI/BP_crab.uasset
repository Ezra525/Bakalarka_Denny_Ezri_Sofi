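; BP_crab is a possessable crab that the player uses to open lab doors and vents.
; Pressing E runs a door check on overlapping BP_LABdoor1 actors, then line traces from the follow camera to open a hit BP_vent tagged "vent".
; When unpossessed, it spawns its default controller to take over.
; Lifespan and delayed-destroy logic is present but disconnected, so it never runs.
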(event EventBeginPlay)

(event EventUnpossessed
  (params (OldController :type Controller%20Object%20Reference))
  (Pawn|SpawnDefaultController))

(event Input|KeyboardEvents|E
  (params (Key :type Key%20Structure :default "None"))
  (bind _followcamera (Variables|Default|GetFollowCamera))
  (bind _returnvalue (Transformation|GetWorldLocation _followcamera))
  ;[0.15 0.005555 0.04333 0.5] openDoor
  (:Pressed
    (Utilities|FlowControl|Sequence
      (:then_0
        (for _array_element (Collision|GetOverlappingActors 0 :!class /Script/Engine.Actor)
          (bind _asbp_labdoor_1 (Utilities|Casting|CastToBP_LABdoor1 _array_element))
          (Default|OPenDoorCheck _asbp_labdoor_1)))
      (:then_1
        ;[0.15 0.1437 0.01434 0.5] OPen Vent
        (bind (_outhit _returnvalue_2) (Collision|LineTraceByChannel _returnvalue (+ _returnvalue (* (Math|Vector|GetForwardVector _followcamera) 3e+03)) "TraceTypeQuery1" false 0 "None"))
        (if _returnvalue_2
          (if (Actor|ActorHasTag (.HitActor (Collision|BreakHitResult _outhit)) "vent")
            (bind _asbp_vent (Utilities|Casting|CastToBP_vent (.HitActor (Collision|BreakHitResult _outhit))))
            (Default|OpenVent _asbp_vent)))))))

(fn ConstructionScript)