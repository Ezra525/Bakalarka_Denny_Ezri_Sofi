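; Possessable crab character that the player can temporarily control to climb, open doors and vents, and inspect notes.
; Q line-traces for a wall, then switches to plane-constrained flying (marked as not working).
; E interacts via overlaps and a camera trace, showing notes as a mouse-rotatable mesh.
; Timed health drain, lethal damage or Tab returns control to the original pawn; game mode dispatchers trigger possession timing and respawn.
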(event Custom|CustomEvent
  ;[0.009721 0.006049 0.15 0.502] Respawn
  (Transformation|SetActorLocation (stale EventBeginPlay _returnvalue) false false)
  (Rendering|SetActorHiddenInGame false)
  (Variables|/Game/_BachelorsProject/Components/HeathComponent.HeathComponent_C|SetCurrentHealth (Variables|Default|GetHeathComponent) 100))

(event Custom|ClimbingMovementUpdate
  ;[0.03736 0.05665 0.15 0.5] nefungujuci climbing system hepl
  ;;[0.15 0.15 0.15 0.5] climbingmovement?
  (if (Variables|Default|GetisClimbing)
    (Transformation|AddActorWorldOffset self (* (* 2e+02 (Math|Vector|Normalize (Math|Vector|ProjectVectorontoPlane (Pawn|Components|PawnMovement|GetLastInputVector (Variables|Character|GetCharacterMovement)) (Variables|Default|GetWallNormal)) 1.0)) (Utilities|Time|GetWorldDeltaSeconds)) true)))

(event Custom|Oh%20yeah%20Daddy!
  (bind _heathcomponent (Variables|Default|GetHeathComponent))
  (bind _currenthealth (Variables|/Game/_BachelorsProject/Components/HeathComponent.HeathComponent_C|GetCurrentHealth _heathcomponent))
  ;[1 0.01967 0.7197 0.5] Ca you posses me Daddy?
  (Variables|Default|SetAm%20I%20Possesed? true)
  (Utilities|FlowControl|Delay 5.0 :!label _label)
  (Default|Takedamage _heathcomponent 100)
  (Development|PrintString (Utilities|String|ToString(Integer) _currenthealth) true true "(R=0.000000,G=1.000000,B=0.054582,A=1.000000)" 1e+01)
  (if (<= _currenthealth 0)
    (Default|CallNotMeDaddy (Variables|Default|GetEvent%20Dispather%20God) (Utilities|String|StringToName (Variables|Default|GetI%20have%20name%20bitch!)))
    (if (Variables|Default|Getposses)
      (bind _asbp_third_person_game_mode (Utilities|Casting|CastToBP_ThirdPersonGameMode (Game|GetGameMode)))
      (Pawn|Possess (Game|GetPlayerController 0) (Variables|/Game/ThirdPerson/Blueprints/BP_ThirdPersonGameMode.BP_ThirdPersonGameMode_C|GetOriginalTypek _asbp_third_person_game_mode))
      (Variables|Default|SetAm%20I%20Possesed? false)
      (Utilities|FlowControl|Delay 5.0)
      (Default|ResetHealthinComponent (Variables|Default|GetHeathComponent))
      (Development|PrintString "Hello"))
    (elif (Variables|Default|GetAm%20I%20Possesed?)
      (Development|PrintString "Hi]")
      (goto _label))))

(event Game|Damage|EventAnyDamage
  (params (Damage :type Float%20%28single-precision%29) (DamageType :type Damage%20Type%20Object%20Reference) (InstigatedBy :type Controller%20Object%20Reference) (DamageCauser :type Actor%20Object%20Reference))
  ;[0.15 0.15 0.15 0.5] Unposses ondeath
  (bind _sheathdepleted (Default|Takedamage (Variables|Default|GetHeathComponent) (Math|Float|Truncate Damage)))
  (if _sheathdepleted
    (bind _asbp_third_person_game_mode (Utilities|Casting|CastToBP_ThirdPersonGameMode (Game|GetGameMode)))
    (Pawn|UnPossess (Game|GetPlayerController 0))
    (Pawn|Possess (Game|GetPlayerController 0) (Variables|/Game/ThirdPerson/Blueprints/BP_ThirdPersonGameMode.BP_ThirdPersonGameMode_C|GetOriginalTypek _asbp_third_person_game_mode))
    (Rendering|SetActorHiddenInGame self true)))

(event EventBeginPlay
  ;[0.009721 0.006049 0.15 0.502] Respawn
  (Variables|Default|Setposses false)
  (bind _returnvalue (Transformation|GetActorLocation))
  (bind _asbp_third_person_game_mode (Utilities|Casting|CastToBP_ThirdPersonGameMode (Game|GetGameMode)))
  (Variables|Default|SetEvent%20Dispather%20God _asbp_third_person_game_mode)
  (Utilities|FlowControl|Sequence
    (:then_0
      (EventDispatchers|BindEventtoOnPlayerDeath _asbp_third_person_game_mode (delegate Custom|CustomEvent)))
    (:then_1
      ;[1 0.01967 0.7197 0.5] Ca you posses me Daddy?
      (EventDispatchers|BindEventtoIPossesYou!!! _asbp_third_person_game_mode (delegate Custom|Oh%20yeah%20Daddy!)))))

(event EventUnpossessed
  (params (OldController :type Controller%20Object%20Reference))
  ;[0.15 0.15 0.15 0.5] Unpossesed AI <--> Default controller
  (Utilities|FlowControl|Sequence
    (:then_0
      (Pawn|SpawnDefaultController))
    (:then_1
      (Variables|Default|Setposses false))))

(event EventPossessed
  (params (NewController :type Controller%20Object%20Reference))
  ;[0.15 0.15 0.15 0.5] Unpossesed AI <--> Default controller
  (Variables|Default|Setposses true))

(event Input|MouseEvents|MouseX
  (params (AxisValue :type Float%20%28single-precision%29))
  (bind _e (Variables|Default|Gete))
  (if (stale Input|KeyboardEvents|E _output_get)
    (Transformation|SetWorldTransform _e (Math|Transform|MakeTransform (Transformation|GetWorldLocation _e) (Math|Rotator|CombineRotators (Transformation|GetWorldRotation _e) (Math|Rotator|MakeRotator 0.0 0.0 AxisValue)) "1.000000,1.000000,1.000000") false false)))

(event Input|KeyboardEvents|Tab
  (params (Key :type Key%20Structure :default "None"))
  ;[1 0.01967 0.7197 0.5] Ca you posses me Daddy?
  (:Pressed
    (if (Variables|Default|Getposses)
      (bind _asbp_third_person_game_mode (Utilities|Casting|CastToBP_ThirdPersonGameMode (Game|GetGameMode)))
      (Pawn|Possess (Game|GetPlayerController 0) (Variables|/Game/ThirdPerson/Blueprints/BP_ThirdPersonGameMode.BP_ThirdPersonGameMode_C|GetOriginalTypek _asbp_third_person_game_mode))
      (Variables|Default|SetAm%20I%20Possesed? false)
      (Utilities|FlowControl|Delay 5.0)
      (Default|ResetHealthinComponent (Variables|Default|GetHeathComponent))
      (Development|PrintString "Hello"))))

(event Input|KeyboardEvents|Q
  (params (Key :type Key%20Structure :default "None"))
  (bind _charactermovement (Variables|Character|GetCharacterMovement))
  ;[0.03736 0.05665 0.15 0.5] nefungujuci climbing system hepl
  (:Pressed
    (bind (_outhit _hashit) (CallFunction|ClimbingLineTrace))
    (if _hashit
      (Variables|Default|SetisClimbing true)
      (Transformation|SetActorLocation self (+ (.ImpactPoint (Collision|BreakHitResult _outhit)) (* 1e+01 (Variables|Default|GetImpact%20Normal))) true false)
      (Class|MovementComponent|SetPlaneConstraintEnabled _charactermovement true)
      (Class|MovementComponent|SetPlaneConstraintNormal _charactermovement (.Normal (Collision|BreakHitResult _outhit)))
      (Transformation|SetActorRotation self (Math|Conversions|RotationFromXVector (* (Variables|Default|GetImpact%20Normal) -1.0)))
      (Variables|Default|SetWallNormal (.Normal (Collision|BreakHitResult _outhit)))
      (Pawn|Components|CharacterMovement|SetMovementMode (Variables|Character|GetCharacterMovement) "MOVE_Flying" 0)
      (Variables|Default|SetImpact%20Normal (.ImpactNormal (Collision|BreakHitResult _outhit))))))

(event Input|KeyboardEvents|E
  (params (Key :type Key%20Structure :default "None"))
  (bind _e (Variables|Default|Gete))
  (bind _e_2 (Variables|Default|Gete))
  (bind _followcamera (Variables|Default|GetFollowCamera))
  (bind _returnvalue (Transformation|GetWorldLocation _followcamera))
  ;[0.15 0.005555 0.04333 0.5] openDoor
  (:Pressed
    (Utilities|FlowControl|Sequence
      (:then_0
        (for _array_element (Collision|GetOverlappingActors 0 :!class /Script/Engine.Actor)
          (bind _asbp_labdoor_1 (Utilities|Casting|CastToBP_LABdoor1 _array_element))
          (Default|OPenDoorCheck _asbp_labdoor_1)))
      (:then_1
        (for _array_element_2 (Collision|GetOverlappingActors "/Game/_BachelorsProject/Assets/Blueprints/notes/BP_tabletnotes.BP_tabletnotes_C" :!class /Script/Engine.Actor)
          (if (Utilities|DoesObjectImplementInterface _array_element_2 "/Game/ThirdPerson/Blueprints/BP_INTERACT.BP_INTERACT_C")
            (bind _itemmodell (Class|BPINTERACT|Interactitem(Message) _array_element_2))
            (Components|StaticMesh|SetStaticMesh _e_2 _itemmodell)
            (Rendering|SetVisibility _e_2 true false)
            (bind _output_get (Variables|Default|SetIsViewingItem? true))
            (Components|Activation|Deactivate (Variables|Character|GetCharacterMovement))
            (Components|Activation|Deactivate (Variables|Default|GetCameraBoom))
            (bind _asbp_third_person_game_mode (Utilities|Casting|CastToBP_ThirdPersonGameMode (Game|GetGameMode)))
            (Default|CallCannotUnposses _asbp_third_person_game_mode)
            (Transformation|SetWorldTransform _e (Math|Transform|MakeTransform (Transformation|GetWorldLocation (Variables|Default|Gete)) (Math|Rotator|FindLookatRotation (Transformation|GetWorldLocation _e) (Transformation|GetWorldLocation (Variables|Default|GetCameraBoom))) "1.000000,1.000000,1.000000") false false))))
      (:then_2
        ;[0.15 0.1437 0.01434 0.5] OPen Vent
        (bind (_outhit _returnvalue_2) (Collision|LineTraceByChannel _returnvalue (+ _returnvalue (* (Math|Vector|GetForwardVector _followcamera) 3e+03)) "TraceTypeQuery1" false 0 "None"))
        (if _returnvalue_2
          (if (Actor|ActorHasTag (|CollapseGraph _outhit) "vent")
            (bind _asbp_vent (Utilities|Casting|CastToBP_vent (|CollapseGraph _outhit)))
            (Default|OpenVent _asbp_vent)))))))

(event Input|KeyboardEvents|SpaceBar
  (params (Key :type Key%20Structure :default "None"))
  (:Pressed
    (if (Variables|Default|GetIsViewingItem?)
      (Rendering|SetVisibility (Variables|Default|Gete) false false)
      (Components|Activation|Activate (Variables|Character|GetCharacterMovement) false)
      (Components|Activation|Activate (Variables|Default|GetCameraBoom) false)
      (Variables|Default|SetIsViewingItem? false)
      (bind _asbp_third_person_game_mode (Utilities|Casting|CastToBP_ThirdPersonGameMode (Game|GetGameMode)))
      (Default|CallCanUnposses _asbp_third_person_game_mode))))

(fn ConstructionScript)

(fn ClimbingLineTrace
  (bind _returnvalue (Transformation|GetActorLocation))
  (bind (_outhit _returnvalue_2) (Collision|LineTraceByChannel _returnvalue (+ _returnvalue (* (Math|Vector|GetForwardVector (Transformation|GetActorRotation)) 1e+02)) "TraceTypeQuery1" false 0 "ForDuration"))
  (return _outhit _returnvalue_2))

(fn GetPossesionduration
  (return (Variables|Default|GetpossesionTime_0)))

(fn MyNameIs
  (return (Utilities|String|StringToName (Variables|Default|GetI%20have%20name%20bitch!))))