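; BP_Trigger_Game_Save is a one-shot trigger volume that starts an internal dialogue when the player enters it.
; BeginPlay caches the third-person game mode, and the Box overlap passes the InternalDialogue variable to its CallInternalDialogue, then sets Triggered to block repeats.
; Despite the asset name, the graph contains no save logic.
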(event OnComponentBeginOverlap(Box)
  (params (OverlappedComponent :type Primitive%20Component%20Object%20Reference) (OtherActor :type Actor%20Object%20Reference) (OtherComp :type Primitive%20Component%20Object%20Reference) (OtherBodyIndex :type Integer) (bFromSweep :type Boolean) (SweepResult :type Hit%20Result%20Structure%20%28by%20ref%29))
  (if (not (Variables|Default|GetTriggered?))
    (if (== OtherActor (Game|GetPlayerCharacter 0))
      (Default|CallInternalDialogue (Variables|Default|GetAs%20BP%20Third%20Person%20Game%20Mode) (Variables|Default|GetInternal%20Dialogue))
      (Variables|Default|SetTriggered? true))))

(event EventBeginPlay
  (bind _asbp_third_person_game_mode (Utilities|Casting|CastToBP_ThirdPersonGameMode (Game|GetGameMode)))
  (Variables|Default|SetAs%20BP%20Third%20Person%20Game%20Mode _asbp_third_person_game_mode))

(fn ConstructionScript)