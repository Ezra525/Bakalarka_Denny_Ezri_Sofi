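; Checkpoint trigger that saves the player's progress when their character first overlaps its box.
; It loads the existing save from a fixed slot, writes the character's location and current level name into it, then saves it back.
; A flag blocks repeat saves after one succeeds, and nothing is saved if the load or cast fails.
; The game mode reference cached on BeginPlay is not used by the save.
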(event OnComponentBeginOverlap(Box)
  (params (OverlappedComponent :type Primitive%20Component%20Object%20Reference) (OtherActor :type Actor%20Object%20Reference) (OtherComp :type Primitive%20Component%20Object%20Reference) (OtherBodyIndex :type Integer) (bFromSweep :type Boolean) (SweepResult :type Hit%20Result%20Structure%20%28by%20ref%29))
  (if (not (Variables|Default|GetTriggered?))
    (if (== OtherActor (Game|GetPlayerCharacter 0))
      (bind _returnvalue (SaveGame|LoadGamefromSlot "Slot1"))
      (bind _asbp_save_game (Utilities|Casting|CastToBP_SaveGame _returnvalue))
      (Variables|/Game/_BachelorsProject/Assets/Blueprints/GUI/MainMenu/save/BP_SaveGame.BP_SaveGame_C|SetCheckpoint%20Location _asbp_save_game (Transformation|GetActorLocation (Game|GetPlayerCharacter 0)))
      (bind _returnvalue_2 (Game|GetCurrentLevelName true))
      (Variables|/Game/_BachelorsProject/Assets/Blueprints/GUI/MainMenu/save/BP_SaveGame.BP_SaveGame_C|SetLevel _asbp_save_game (Utilities|String|StringToName _returnvalue_2))
      (SaveGame|SaveGametoSlot _asbp_save_game "Slot1")
      (Development|PrintString "Called save game" true true "(R=1.000000,G=0.000000,B=0.986404,A=1.000000)")
      (Variables|Default|SetTriggered? true))))

(event EventBeginPlay
  (bind _asbp_third_person_game_mode (Utilities|Casting|CastToBP_ThirdPersonGameMode (Game|GetGameMode)))
  (Variables|Default|SetAs%20BP%20Third%20Person%20Game%20Mode _asbp_third_person_game_mode))

(fn ConstructionScript)