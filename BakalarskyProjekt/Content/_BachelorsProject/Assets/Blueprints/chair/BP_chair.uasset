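; BP_chair is a pushable chair that, once far enough along X, enables collision on three invisible stair meshes.
; On any hit, it rounds the hitter's forward vector and box-traces that direction for obstacles.
; If clear, it disables player movement, attaches the player and slides one step via timeline.
; It then detaches the player in Flying mode and checks X, enabling the stairs after a delay.
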(event Custom|push
  (Variables|Default|Setcurrent%20location (Transformation|GetActorLocation))
  (bind _position (Timeline|Push%20block Play)
    (:Update
      (Transformation|SetActorRelativeLocation (+ (Variables|Default|Getcurrent%20location) (* _position (Variables|Default|Getpushable%20location) (Variables|Default|Gettravel%20instance)))))
    (:Finished
      (CallFunction|StopPushing)
      (CallFunction|BulidStairs))))

(event Custom|stop%20pushing
  (bind _returnvalue (Game|GetPlayerCharacter 0))
  (Pawn|Components|CharacterMovement|SetMovementMode (Variables|/Script/Engine.Character|GetCharacterMovement _returnvalue) "MOVE_Flying" 0)
  (Transformation|DetachFromActor _returnvalue "KeepWorld" "KeepWorld" "KeepWorld"))

(event Custom|bulid%20stairs
  (bind _returnvalue (Transformation|GetActorLocation))
  (bind _returnvalue_2 (>= -7435.0 (.x _returnvalue)))
  (Development|PrintString (Utilities|String|ToString(Boolean) _returnvalue_2))
  (if _returnvalue_2
    (Development|PrintString "starirs are here")
    (Utilities|FlowControl|Delay 5.0)
    (Collision|SetCollisionEnabled (Variables|Default|GetSM_Invisible_Stairs1) "QueryAndPhysics")))

(event EventBeginPlay
  (Collision|SetCollisionEnabled (Variables|Default|GetSM_Invisible_Stairs1) "NoCollision"))

(event Collision|EventHit
  (params (MyComp :type Primitive%20Component%20Object%20Reference) (Other :type Actor%20Object%20Reference) (OtherComp :type Primitive%20Component%20Object%20Reference) (bSelfMoved :type Boolean) (HitLocation :type Vector :default "0, 0, 0") (HitNormal :type Vector :default "0, 0, 0") (NormalImpulse :type Vector :default "0, 0, 0") (Hit :type Hit%20Result%20Structure%20%28by%20ref%29))
  (bind _returnvalue (Transformation|GetActorForwardVector Other))
  (bind _returnvalue_2 (Game|GetPlayerCharacter 0))
  (bind (_x _y _z) (Math|Vector|BreakVector _returnvalue))
  (Variables|Default|Setpushable%20location (Math|Vector|MakeVector (Math|Conversions|ToFloat(Integer) (Math|Float|Round _x)) (Math|Conversions|ToFloat(Integer) (Math|Float|Round _y)) (Math|Conversions|ToFloat(Integer) (Math|Float|Round _z))))
  (bind _can_push (CallFunction|CanPush))
  (if _can_push
    (Pawn|Components|CharacterMovement|DisableMovement (Variables|/Script/Engine.Character|GetCharacterMovement _returnvalue_2))
    (Transformation|AttachActorToActor _returnvalue_2 self "None" "KeepWorld" "KeepWorld" "KeepWorld" true)
    (CallFunction|Push)))

(fn ConstructionScript)

(fn CanPush
  (bind _returnvalue (Transformation|GetActorLocation))
  (bind _r (Variables|Default|Getr))
  (bind _staticmesh (Variables|/Script/Engine.StaticMeshComponent|GetStaticMesh _r))
  (bind _returnvalue_2 (StaticMesh|GetBounds _staticmesh))
  (bind _returnvalue_3 (Class|KismetSystemLibrary|BoxTraceMulti (+ _returnvalue (Math|Vector|MakeVector 0.0 0.0 0.0)) (+ _returnvalue (* (Variables|Default|Getpushable%20location) (Variables|Default|Gettravel%20instance)) (.boxextent _returnvalue_2) (Math|Vector|MakeVector 0.0 0.0 0.0)) (.boxextent _returnvalue_2) "0, 0, 0" "TraceTypeQuery1" false 0 "None" true))
  (return (not _returnvalue_3)))