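; BP_chair2 is a pushable chair that, once shoved far enough, makes invisible stairs solid.
; A character hit snaps its forward vector to whole-number axes and box-traces the destination for obstacles.
; If clear, the character is frozen and attached while a timeline slides the chair, then released.
; After each push, reaching a hard-coded world Y threshold enables the three stair meshes' collision after a delay.
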(event OnActorHit(charakter)
  (params (SelfActor :type Actor%20Object%20Reference) (OtherActor :type Actor%20Object%20Reference) (NormalImpulse :type Vector :default "0, 0, 0") (Hit :type Hit%20Result%20Structure%20%28by%20ref%29))
  (bind _returnvalue (Transformation|GetActorForwardVector SelfActor))
  (bind _charakter (Variables|Default|Getcharakter))
  (bind (_x _y) (Math|Vector|BreakVector _returnvalue))
  (if (== self OtherActor)
    (Variables|Default|Setpushable%20location (Math|Vector|MakeVector (Math|Conversions|ToFloat(Integer) (Math|Float|Round _x)) (Math|Conversions|ToFloat(Integer) (Math|Float|Round _y)) 0.0))
    (bind _can_push (CallFunction|CanPush))
    (if _can_push
      (Pawn|Components|CharacterMovement|DisableMovement (Variables|/Script/Engine.Character|GetCharacterMovement _charakter))
      (Transformation|AttachActorToActor _charakter self "None" "KeepWorld" "KeepWorld" "KeepWorld" true)
      (CallFunction|Push)
      (else
        (Development|PrintString "Hello")))))

(event Custom|push
  (Variables|Default|Setcurrent%20location (Transformation|GetActorLocation))
  (bind _position (Timeline|Push%20block Play)
    (:Update
      (Transformation|SetActorRelativeLocation (+ (Variables|Default|Getcurrent%20location) (* _position (Variables|Default|Getpushable%20location) (Variables|Default|Gettravel%20instance)))))
    (:Finished
      (CallFunction|StopPushing)
      (CallFunction|BulidStairs))))

(event Custom|stop%20pushing
  (bind _charakter (Variables|Default|Getcharakter))
  (Pawn|Components|CharacterMovement|SetMovementMode (Variables|/Script/Engine.Character|GetCharacterMovement _charakter) "MOVE_Walking" 0)
  (Transformation|DetachFromActor _charakter "KeepWorld" "KeepWorld" "KeepWorld"))

(event Custom|bulid%20stairs
  (bind _returnvalue (Transformation|GetActorLocation))
  (bind _returnvalue_2 (>= -3839.0 (.y _returnvalue)))
  (Development|PrintString (Utilities|String|ToString(Boolean) _returnvalue_2))
  (if _returnvalue_2
    (Development|PrintString "starirs are here")
    (Utilities|FlowControl|Delay 5.0)
    (Collision|SetCollisionEnabled (Variables|Default|GetSM_Invisible_Stairs1) "QueryAndPhysics")))

(event EventBeginPlay
  (Collision|SetCollisionEnabled (Variables|Default|GetSM_Invisible_Stairs1) "NoCollision"))

(fn ConstructionScript)

(fn CanPush
  (bind _returnvalue (Transformation|GetActorLocation))
  (bind _r (Variables|Default|Getr))
  (bind _staticmesh (Variables|/Script/Engine.StaticMeshComponent|GetStaticMesh _r))
  (bind _returnvalue_2 (StaticMesh|GetBounds _staticmesh))
  (bind _returnvalue_3 (Class|KismetSystemLibrary|BoxTraceMulti _returnvalue (+ _returnvalue (* (Variables|Default|Getpushable%20location) (Variables|Default|Gettravel%20instance)) (.boxextent _returnvalue_2) "") (- (.boxextent _returnvalue_2) "2.000000,2.000000,1.000000") "0, 0, 0" "TraceTypeQuery1" false (Utilities|Array|MakeArray (Variables|Default|Getcharakter)) "None" true))
  (return (not _returnvalue_3)))