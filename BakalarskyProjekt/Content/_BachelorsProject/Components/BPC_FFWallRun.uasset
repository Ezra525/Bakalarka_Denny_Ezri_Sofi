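; Wall-run component that lets the third-person character latch onto and run along surfaces using custom gravity.
; Left Shift traces forward, then blends the capsule to an angle-based orientation and sets gravity against the hit normal.
; A looping timer re-traces downward to update gravity, while a lost surface, forward box-trace hit or IA_Swim detaches and restores gravity.
; Actors tagged "Sphere" get special exit rotation and optional player-following camera.
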(event Custom|OffWall
  (bind _character (Variables|Default|GetCharacter))
  (bind _character_2 (Variables|Default|GetCharacter))
  (bind _character_3 (Variables|Default|GetCharacter))
  (bind _character_4 (Variables|Default|GetCharacter))
  (bind _returnvalue (Transformation|GetActorForwardVector _character))
  (bind _charactermovement (Variables|/Script/Engine.Character|GetCharacterMovement _character_3))
  (bind _returnvalue_2 (Utilities|Operators|EqualEqual _returnvalue "0.000000,0.000000,1.000000" 0.4))
  (Utilities|Time|ClearandInvalidateTimerbyHandle (Variables|Default|GetUpdateGravityTimer))
  (Variables|Default|SetOnWall false)
  (Variables|/Script/Engine.SceneComponent|SetbAbsoluteRotation (Variables|/Game/ThirdPerson/Blueprints/BP_ThirdPersonCharacter.BP_ThirdPersonCharacter_C|GetCameraBoom _character_2) true)
  (Components|MoveComponentTo (Variables|/Script/Engine.Character|GetCapsuleComponent _character_2) (+ (Transformation|GetActorLocation _character_4) (* (Transformation|GetActorForwardVector _character_4) (Math|Float|SelectFloat 2.5e+02 1.5e+02 _returnvalue_2)) (Math|Vector|MakeVector 0.0 0.0 (Math|Float|SelectFloat 85.0 0.0 (Variables|Default|GetHit)))) (Math|Rotator|SelectRotator (Math|Conversions|RotationFromXVector (Transformation|GetActorUpVector _character)) (Math|Rotator|SelectRotator (Math|Conversions|RotationFromXVector (Transformation|GetActorUpVector _character)) (Math|Conversions|RotationFromXVector (* (Transformation|GetActorUpVector _character) -1.0)) (Variables|Default|GetHit)) (Variables|Default|GetOnSphere)) false false (Math|Float|SelectFloat 0.35 0.25 _returnvalue_2) true)
  (Variables|/Script/Engine.SceneComponent|SetbAbsoluteRotation (Variables|/Game/ThirdPerson/Blueprints/BP_ThirdPersonCharacter.BP_ThirdPersonCharacter_C|GetCameraBoom _character_3) false)
  (Class|CharacterMovementComponent|SetGravityDirection _charactermovement (Math|Vector|MakeVector 0.0 0.0 -1.0)) ; Return gravity to normal
  (Variables|/Script/Engine.CharacterMovementComponent|SetMaxWalkSpeed _charactermovement (Variables|Default|GetDefaultMaxWalkSpeed))
  (Variables|Default|SetOnSphere false)
  (|CameraReset)
  (Variables|Default|SetHit false))

(event Custom|UpdateGravity
  (bind _character (Variables|Default|GetCharacter))
  (bind _returnvalue (Transformation|GetActorLocation _character))
  ;[0.3804 0.9412 1] Update gravity direction
  (bind (_outhit _returnvalue_2) (Collision|LineTraceByChannel _returnvalue (+ _returnvalue (* (Transformation|GetActorUpVector _character) -3e+02)) "TraceTypeQuery1" false 0 "None"))
  (if _returnvalue_2
    (Class|CharacterMovementComponent|SetGravityDirection (Variables|/Script/Engine.Character|GetCharacterMovement (Game|GetPlayerCharacter 0)) (* (.Normal (Collision|BreakHitResult _outhit)) -1.0))
    (else
      (Variables|Default|SetHit false)
      (CallFunction|OffWall))))

(event Input|EnhancedActionEvents|EnhancedInputActionIA_Look
  (params (ActionValue :type Vector%202D%20Structure) (ElapsedSeconds :type Float%20%28double-precision%29) (TriggeredSeconds :type Float%20%28double-precision%29) (InputAction :type Input%20Action%20Object%20Reference :default "/Game/ThirdPerson/Input/Actions/IA_Look.IA_Look"))
  ;[0.3804 0.9412 1] Input Actions and character reference
  (:Triggered
    (Variables|Default|SetRotationScale (/ (.x ActionValue) 3.0)))
  (:Completed
    (Variables|Default|SetRotationScale 0.0)))

(event Input|EnhancedActionEvents|EnhancedInputActionIA_Move
  (params (ActionValue :type Vector%202D%20Structure) (ElapsedSeconds :type Float%20%28double-precision%29) (TriggeredSeconds :type Float%20%28double-precision%29) (InputAction :type Input%20Action%20Object%20Reference :default "/Game/ThirdPerson/Input/Actions/IA_Move.IA_Move"))
  ;[0.3804 0.9412 1] Input Actions and character reference
  (if (Variables|Default|GetOnWall)
    (|WallMovement (.x ActionValue) (.y ActionValue))))

(event Input|EnhancedActionEvents|EnhancedInputActionIA_Swim
  (params (ActionValue :type Float%20%28double-precision%29) (ElapsedSeconds :type Float%20%28double-precision%29) (TriggeredSeconds :type Float%20%28double-precision%29) (InputAction :type Input%20Action%20Object%20Reference :default "/Game/ThirdPerson/Input/Actions/IA_Swim.IA_Swim"))
  ;[0.3804 0.9412 1] Input Actions and character reference
  (:Started
    (if (Variables|Default|GetOnWall)
      (CallFunction|OffWall))))

(event EventBeginPlay
  ;[0.3804 0.9412 1] Input Actions and character reference
  (bind _returnvalue (Actor|GetActorOfClass "/Game/ThirdPerson/Blueprints/BP_ThirdPersonCharacter.BP_ThirdPersonCharacter_C"))
  (Variables|Default|SetCharacter _returnvalue))

(event Input|KeyboardEvents|LeftShift
  (params (Key :type Key%20Structure :default "None"))
  (bind _character (Variables|Default|GetCharacter))
  (bind _character_2 (Variables|Default|GetCharacter))
  (bind _character_3 (Variables|Default|GetCharacter))
  (bind _returnvalue (Transformation|GetActorLocation _character_2))
  (bind _charactermovement (Variables|/Script/Engine.Character|GetCharacterMovement _character_3))
  (:Pressed
    (bind (_outhit _returnvalue_2) (Collision|LineTraceByChannel _returnvalue (+ _returnvalue (* (Transformation|GetActorForwardVector _character_2) 2e+02)) "TraceTypeQuery1" false 0 "None"))
    (if _returnvalue_2
      (Character|Jump (Variables|Default|GetCharacter)) ; Jumps to soothe transition\nto the wall.
      (bind (_location _normal _hitactor) (|CalculateWallAngle _outhit))
      (bind _target_relative_location (CallFunction|DetermineLatchAngle _normal _hitactor))
      (Variables|/Script/Engine.SceneComponent|SetbAbsoluteRotation (Variables|/Game/ThirdPerson/Blueprints/BP_ThirdPersonCharacter.BP_ThirdPersonCharacter_C|GetCameraBoom _character) true) ; I had to add this because putting\nthis blueprint into a component\njust started rotating the camera\nand then rotated it back to norrmal.\nSo now you have to deal with having this\nunless you can find a better fix
      (Components|MoveComponentTo (Variables|/Script/Engine.Character|GetCapsuleComponent _character) (+ _location (* _normal 9e+01) "0.000000,0.000000,25.000000") _target_relative_location false false (Variables|Default|GetLatchDuration) true)
      (|SphereOrientation _hitactor)
      (Variables|/Script/Engine.SceneComponent|SetbAbsoluteRotation (Variables|/Game/ThirdPerson/Blueprints/BP_ThirdPersonCharacter.BP_ThirdPersonCharacter_C|GetCameraBoom (Variables|Default|GetCharacter)) false)
      (Variables|Default|SetOnWall true)
      (Class|CharacterMovementComponent|SetGravityDirection _charactermovement (* _normal -1.0)) ; Set gravity to the normal of our hit surface
      (Variables|/Script/Engine.CharacterMovementComponent|SetMaxWalkSpeed _charactermovement (Variables|Default|GetWallRunSpeed))
      (bind _returnvalue_3 (Utilities|Time|SetTimerbyEvent (EventDispatchers|CreateEvent :!event Custom|UpdateGravity) 0.01 true true)) ; Start timer to continuously update gravity direction
      (Variables|Default|SetUpdateGravityTimer _returnvalue_3))))

(fn DetermineLatchAngle
  (params (Hit%20Actor%20Normal :type Vector) (Hit%20Actor :type Actor%20Object%20Reference))
  (bind _returnvalue (Transformation|GetActorUpVector Hit%20Actor))
  (if (< (Variables|Default|GetHitAngle) 6e+01)
    (Variables|Default|SetTarget%20Relative%20Rotation (Math|Rotator|MakeRotfromZY Hit%20Actor%20Normal _returnvalue))
    (elif (> (Variables|Default|GetHitAngle) 1.2e+02)
      (Variables|Default|SetTarget%20Relative%20Rotation (Math|Rotator|MakeRotfromZY Hit%20Actor%20Normal (* _returnvalue -1.0)))
      (else
        (Variables|Default|SetTarget%20Relative%20Rotation (Math|Rotator|MakeRotfromZX Hit%20Actor%20Normal _returnvalue)))))
  (return (Variables|Default|GetTarget%20Relative%20Rotation)))