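; BP_StaircaseDebree is a staircase debris hazard that damages characters on contact and drops out of the level after the player dies.
; Overlapping component R applies 100 damage to "character"-tagged actors that have a HeathComponent, with a DoOnce limiting hits to one per two seconds and a debug print.
; It binds to the ThirdPerson game mode's player death event, then after a delay shifts its root 20000 units down.
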(event OnComponentBeginOverlap(r)
  (params (OverlappedComponent :type Primitive%20Component%20Object%20Reference) (OtherActor :type Actor%20Object%20Reference) (OtherComp :type Primitive%20Component%20Object%20Reference) (OtherBodyIndex :type Integer) (bFromSweep :type Boolean) (SweepResult :type Hit%20Result%20Structure%20%28by%20ref%29))
  (if (Actor|ActorHasTag OtherActor "character")
    (Utilities|IsValid (Actor|GetComponentbyClass OtherActor "/Game/_BachelorsProject/Components/HeathComponent.HeathComponent_C")
      (:Is%20Valid
        (Utilities|FlowControl|DoOnce false :!label _label
          (:Completed
            (bind _returnvalue (Game|Damage|ApplyDamage OtherActor 1e+02 0 0))
            (Development|PrintString (Utilities|String|ToString(Float) _returnvalue) true true "(R=1.000000,G=0.782915,B=0.000000,A=1.000000)" 1e+01)
            (Utilities|FlowControl|Delay 2.0)
            (goto _label Reset)))))))

(event Custom|OnPlayerDeath_Event
  (Utilities|FlowControl|Delay 2.0)
  (Transformation|AddRelativeLocation (Variables|Default|GetDefaultSceneRoot) "0.000000,0.000000,-20000.000000" false false))

(event EventBeginPlay
  (bind _asbp_third_person_game_mode (Utilities|Casting|CastToBP_ThirdPersonGameMode (Game|GetGameMode)))
  (EventDispatchers|AssignOnPlayerDeath _asbp_third_person_game_mode (delegate Custom|OnPlayerDeath_Event)))

(fn ConstructionScript)